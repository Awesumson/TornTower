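; Healing spring Blueprint that restores the player's health while they stand inside its sphere trigger.
; Sphere overlap events cast to ThirdPersonCharacterTT and toggle an overlap flag, with begin overlap also storing the character and starting HealDelay.
; HealDelay re-calls itself after each short delay, adding health with no upper limit.
; The flag is checked before the delay, so a pending heal still lands after exit.
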(event OnComponentBeginOverlap(Sphere)
  (params (OverlappedComponent :type Primitive%20Component%20Object%20Reference) (OtherActor :type Actor%20Object%20Reference) (OtherComp :type Primitive%20Component%20Object%20Reference) (OtherBodyIndex :type Integer) (bFromSweep :type Boolean) (SweepResult :type Hit%20Result%20Structure%20%28by%20ref%29))
  (bind _asthird_person_character_tt (Utilities|Casting|CastToThirdPersonCharacterTT OtherActor))
  (Variables|Default|SetIsOverlappedByPlayer true)
  (CallFunction|HealDelay))

(event OnComponentEndOverlap(Sphere)
  (params (OverlappedComponent :type Primitive%20Component%20Object%20Reference) (OtherActor :type Actor%20Object%20Reference) (OtherComp :type Primitive%20Component%20Object%20Reference) (OtherBodyIndex :type Integer))
  (Utilities|Casting|CastToThirdPersonCharacterTT OtherActor)
  (Variables|Default|SetIsOverlappedByPlayer false))

(event Custom|Heal%20Delay
  (if (Variables|Default|GetIsOverlappedByPlayer)
    (Utilities|FlowControl|Delay 2.0)
    (Variables|/Game/GameBPs/Blueprints/ThirdPersonCharacterTT.ThirdPersonCharacterTT_C|SetTotalHealth (stale OnComponentBeginOverlap(Sphere) _asthird_person_character_tt) (+ (Variables|/Game/GameBPs/Blueprints/ThirdPersonCharacterTT.ThirdPersonCharacterTT_C|GetTotalHealth (stale OnComponentBeginOverlap(Sphere) _asthird_person_character_tt)) 1))
    (CallFunction|HealDelay)))

(fn ConstructionScript)