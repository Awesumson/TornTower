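; Test ladder actor that switches a ThirdPersonCharacterTT into and out of ladder climbing through its ClimbVolume overlaps.
; Entering while moving above a small speed threshold sets the climbing flag and passes the ladder's location; entering while already climbing clears it and zeroes rotation.
; Leaving clears the flag, then tests it, so the following mesh-clearing call on Ladder is effectively unreachable.
; The climbing movement itself is not handled here.
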(event OnComponentBeginOverlap(ClimbVolume)
  (params (OverlappedComponent :type Primitive%20Component%20Object%20Reference) (OtherActor :type Actor%20Object%20Reference) (OtherComp :type Primitive%20Component%20Object%20Reference) (OtherBodyIndex :type Integer) (bFromSweep :type Boolean) (SweepResult :type Hit%20Result%20Structure%20%28by%20ref%29))
  (bind _outactors (Actor|GetAllActorsOfClass 0))
  (bind _asthird_person_character_tt (Utilities|Casting|CastToThirdPersonCharacterTT OtherActor))
  (if (Variables|/Game/GameBPs/Blueprints/ThirdPersonCharacterTT.ThirdPersonCharacterTT_C|GetIsClimbingLadder _asthird_person_character_tt)
    (Variables|/Game/GameBPs/Blueprints/ThirdPersonCharacterTT.ThirdPersonCharacterTT_C|SetIsClimbingLadder _asthird_person_character_tt false)
    (Transformation|SetActorRotation _asthird_person_character_tt)
    (elif (> (Math|Vector|VectorLength (Transformation|GetVelocity _asthird_person_character_tt)) 1e+01)
      (Variables|/Game/GameBPs/Blueprints/ThirdPersonCharacterTT.ThirdPersonCharacterTT_C|SetIsClimbingLadder _asthird_person_character_tt true)
      (Variables|/Game/GameBPs/Blueprints/ThirdPersonCharacterTT.ThirdPersonCharacterTT_C|SetLadderPosition _asthird_person_character_tt (Transformation|GetActorLocation)))))

(event OnComponentEndOverlap(ClimbVolume)
  (params (OverlappedComponent :type Primitive%20Component%20Object%20Reference) (OtherActor :type Actor%20Object%20Reference) (OtherComp :type Primitive%20Component%20Object%20Reference) (OtherBodyIndex :type Integer))
  (bind _asthird_person_character_tt (Utilities|Casting|CastToThirdPersonCharacterTT OtherActor))
  (bind _output_get (Variables|/Game/GameBPs/Blueprints/ThirdPersonCharacterTT.ThirdPersonCharacterTT_C|SetIsClimbingLadder _asthird_person_character_tt false))
  (if _output_get
    (Components|StaticMesh|SetStaticMesh (Variables|Default|GetLadder) 0)))

(fn ConstructionScript)