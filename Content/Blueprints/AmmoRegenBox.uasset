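; AmmoRegenBox is a pickup actor that grants the player ammo and starts ammo regeneration when a ThirdPersonCharacter overlaps it.
; The overlap adds a fixed amount of Ammo, sets AmmoRegenActive, calls the character's AmmoRegen, then destroys the box.
; It also shows an AmmoRegenCollected widget, gated by the character's PopupDisplayed flag to avoid repeat popups, and calls ResetPopup on the character.
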(event Collision|EventActorBeginOverlap
  (params (OtherActor :type Actor%20Object%20Reference))
  (bind _asthird_person_character (Utilities|Casting|CastToThirdPersonCharacter OtherActor))
  (Variables|/Game/GameBPs/Blueprints/ThirdPersonCharacter.ThirdPersonCharacter_C|SetAmmo _asthird_person_character (+ (Variables|/Game/GameBPs/Blueprints/ThirdPersonCharacter.ThirdPersonCharacter_C|GetAmmo _asthird_person_character) 5))
  (Variables|/Game/GameBPs/Blueprints/ThirdPersonCharacter.ThirdPersonCharacter_C|SetAmmoRegenActive? _asthird_person_character true)
  (Default|AmmoRegen _asthird_person_character)
  (Actor|DestroyActor)
  (if (not (Variables|/Game/GameBPs/Blueprints/ThirdPersonCharacter.ThirdPersonCharacter_C|GetPopupDisplayed? _asthird_person_character))
    (Variables|/Game/GameBPs/Blueprints/ThirdPersonCharacter.ThirdPersonCharacter_C|SetPopupDisplayed? _asthird_person_character true)
    (Default|ResetPopup _asthird_person_character)
    (bind _returnvalue (UserInterface|CreateWidget "/Game/Interfaces/AmmoRegenCollected.AmmoRegenCollected_C" (Game|GetPlayerController 0)))
    (UserInterface|Viewport|AddtoViewport _returnvalue 0)))

(fn ConstructionScript)