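; Startup Blueprint that kicks off enemy spawning for the Basic, Suicide, Destroyer and Stalker AI types.
; TriggerSpawns calls one custom event per type, each finding every matching EnemySpawn actor in the level and calling its PickSpawnTime.
; It then prints spawn and airdrop start messages, though no airdrop logic runs here.
; Nothing in this Blueprint calls TriggerSpawns itself.
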(event Custom|TriggerSpawns
  (CallFunction|TriggerBasicAI)
  (CallFunction|TriggerSuicideAI)
  (CallFunction|TriggerDestroyerAI)
  (CallFunction|TriggerStalkerAI)
  (Development|PrintString "Spawns started..." true true "(R=0.000000,G=0.660000,B=1.000000,A=1.000000)" 5.0)
  (Development|PrintString "Airdrops started..." true true "(R=0.000000,G=0.660000,B=1.000000,A=1.000000)" 5.0))

(event Custom|TriggerStalkerAI
  (bind _outactors (Actor|GetAllActorsOfClass "/Game/Blueprints/EnemySpawn_Stalker.EnemySpawn_Stalker_C"))
  (for _array_element _outactors
    (Default|PickSpawnTime _array_element)))

(event Custom|TriggerSuicideAI
  (bind _outactors (Actor|GetAllActorsOfClass "/Game/Blueprints/EnemySpawn_Suicide.EnemySpawn_Suicide_C"))
  (for _array_element _outactors
    (Default|PickSpawnTime _array_element)))

(event Custom|TriggerDestroyerAI
  (bind _outactors (Actor|GetAllActorsOfClass "/Game/Blueprints/EnemySpawn_Destroyer.EnemySpawn_Destroyer_C"))
  (for _array_element _outactors
    (Default|PickSpawnTime _array_element)))

(event Custom|TriggerBasicAI
  (bind _outactors (Actor|GetAllActorsOfClass "/Game/Blueprints/EnemySpawn_Basic.EnemySpawn_Basic_C"))
  (for _array_element _outactors
    (Default|PickSpawnTime _array_element)))

(fn ConstructionScript)