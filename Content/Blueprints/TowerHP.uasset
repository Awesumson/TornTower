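; TowerHP tracks a tower's health and removes the player-character class actors when that health runs out.
; TakeDamage sets a cast-success flag, subtracts a fixed amount and calls HealthCheck, which destroys every ThirdPersonCharacterTT actor at zero or below.
; Tick caps health at a hard-coded maximum every frame.
; A debug print of LastHealthAddition is left unconnected and never runs.
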(event Custom|TakeDamage
  (Variables|Default|SetCast%20Sucessful? true)
  (Variables|Default|SetTowerHealth (- (Variables|Default|GetTowerHealth) 5))
  (CallFunction|HealthCheck))

(event Custom|HealthCheck
  (if (<= (Variables|Default|GetTowerHealth) 0)
    (bind _outactors (Actor|GetAllActorsOfClass "/Game/GameBPs/Blueprints/ThirdPersonCharacterTT.ThirdPersonCharacterTT_C"))
    (for _array_element _outactors
      (Actor|DestroyActor _array_element))))

(event EventTick
  (params (DeltaSeconds :type Float%20%28single-precision%29))
  (if (>= (Variables|Default|GetTowerHealth) 1500)
    (Variables|Default|SetTowerHealth 1500)))

(fn ConstructionScript)