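; Friendly stalker mine that detonates shortly after an Enemy-tagged actor overlaps it, or when damage depletes its health.
; Overlap spawns a short-lived ExplosionShotRadius and debug sphere, then joins the health path's explosion effect, sound and destroy.
; A self-recursing delayed event, started once from Tick, blinks the point light.
; ReduceSpawnCount decrements MinesSpawned on the first StalkerAI_laser found in the level.
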(event Custom|Health%20Check
  (bind _cylinder (Variables|Default|GetCylinder))
  (bind _returnvalue (Transformation|GetWorldLocation _cylinder))
  (if (<= (Variables|Default|GetHealth) 0.0)
    (Utilities|FlowControl|DoOnce false
      (:Completed
        (Effects|SpawnEmitteratLocation "/Game/StarterContent/Particles/P_Explosion.P_Explosion" _returnvalue "0, 0, 0" "4.000000,4.000000,4.000000")
        (Game|SpawnActorfromClass "/Game/ExplosionSFX.ExplosionSFX_C" (Math|Conversions|ToTransform(Vector) _returnvalue) "Undefined" 0 0)
        (Actor|DestroyActor)))))

(event Custom|ReduceSpawnCount
  (params (DestroyedActor :type Actor%20Object%20Reference))
  (bind _outactors (Actor|GetAllActorsOfClass "/Game/GameBPs/Blueprints/StalkerAI_laser.StalkerAI_laser_C"))
  (Variables|/Game/GameBPs/Blueprints/StalkerAI_laser.StalkerAI_laser_C|SetMinesSpawned (Utilities|Array|Get(acopy) _outactors) (- (Variables|/Game/GameBPs/Blueprints/StalkerAI_laser.StalkerAI_laser_C|GetMinesSpawned (Utilities|Array|Get(acopy) _outactors)) 1)))

(event Custom|Mine%20Lights
  (Rendering|Components|Light|SetLightColor (Variables|Default|GetPointLight) (Variables|Default|GetLightOn) true)
  (Utilities|FlowControl|Delay 0.5)
  (Rendering|Components|Light|SetLightColor (Variables|Default|GetPointLight) (Variables|Default|GetLightOff) true)
  (Utilities|FlowControl|Delay 0.5)
  (CallFunction|MineLights))

(event Collision|EventActorBeginOverlap
  (params (OtherActor :type Actor%20Object%20Reference))
  (bind _cylinder (Variables|Default|GetCylinder))
  (bind _returnvalue (Transformation|GetWorldLocation _cylinder))
  (if (Actor|ActorHasTag OtherActor "Enemy")
    (Utilities|FlowControl|DoOnce false
      (:Completed
        (Utilities|FlowControl|Delay 0.5)
        (bind _returnvalue_2 (Game|SpawnActorfromClass "/Game/Blueprints/ExplosionShotRadius.ExplosionShotRadius_C" (Math|Conversions|ToTransform(Vector) _returnvalue) "Undefined" 0 0))
        (Actor|SetLifeSpan _returnvalue_2 0.5)
        (Rendering|Debug|DrawDebugSphere _returnvalue 3e+02 12 "(R=1.000000,G=0.000000,B=0.008232,A=1.000000)" 1.0 2.0)
        (Effects|SpawnEmitteratLocation "/Game/StarterContent/Particles/P_Explosion.P_Explosion" _returnvalue "0, 0, 0" "4.000000,4.000000,4.000000")
        (Game|SpawnActorfromClass "/Game/ExplosionSFX.ExplosionSFX_C" (Math|Conversions|ToTransform(Vector) _returnvalue) "Undefined" 0 0)
        (Actor|DestroyActor)))))

(event EventTick
  (params (DeltaSeconds :type Float%20%28single-precision%29))
  (Utilities|FlowControl|DoOnce false
    (:Completed
      (CallFunction|MineLights))))

(event Game|Damage|EventAnyDamage
  (params (Damage :type Float%20%28single-precision%29) (DamageType :type Damage%20Type%20Object%20Reference) (InstigatedBy :type Controller%20Object%20Reference) (DamageCauser :type Actor%20Object%20Reference))
  (Variables|Default|SetHealth (- (Variables|Default|GetHealth) Damage))
  (CallFunction|HealthCheck))

(fn ConstructionScript)