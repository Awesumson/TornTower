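; MassFreeze is a pickup actor that triggers a freeze on enemy AI when a ThirdPersonCharacterTT overlaps it.
; Three custom events call MassFreeze on every TowerDestroyerAI, SuicideAI and BasicAI found with GetAllActorsOfClass.
; The pickup then destroys itself and, if the character has no popup displayed, sets that flag, calls ResetPopup and shows the MassFreezeActive widget.
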(event Custom|CastFreezeSuicideAI
  (bind _outactors (Actor|GetAllActorsOfClass "/Game/GameBPs/Blueprints/SuicideAI.SuicideAI_C"))
  (for _array_element _outactors
    (Default|MassFreeze _array_element)))

(event Custom|CastFreezeDestroyerAI
  (bind _outactors (Actor|GetAllActorsOfClass "/Game/GameBPs/Blueprints/TowerDestroyerAI.TowerDestroyerAI_C"))
  (for _array_element _outactors
    (Default|MassFreeze _array_element)))

(event Custom|CastFreezeBasicAi
  (bind _outactors (Actor|GetAllActorsOfClass "/Game/GameBPs/Blueprints/BasicAI.BasicAI_C"))
  (for _array_element _outactors
    (Default|MassFreeze _array_element)))

(event Collision|EventActorBeginOverlap
  (params (OtherActor :type Actor%20Object%20Reference))
  (bind _asthird_person_character_tt (Utilities|Casting|CastToThirdPersonCharacterTT OtherActor))
  (CallFunction|CastFreezeDestroyerAI)
  (CallFunction|CastFreezeSuicideAI)
  (CallFunction|CastFreezeBasicAi)
  (Actor|DestroyActor)
  (if (not (Variables|/Game/GameBPs/Blueprints/ThirdPersonCharacterTT.ThirdPersonCharacterTT_C|GetPopupDisplayed? _asthird_person_character_tt))
    (Variables|/Game/GameBPs/Blueprints/ThirdPersonCharacterTT.ThirdPersonCharacterTT_C|SetPopupDisplayed? _asthird_person_character_tt true)
    (Default|ResetPopup _asthird_person_character_tt)
    (bind _returnvalue (UserInterface|CreateWidget "/Game/Interfaces/MassFreezeActive.MassFreezeActive_C" (Game|GetPlayerController 0)))
    (UserInterface|Viewport|AddtoViewport _returnvalue 0)))

(fn ConstructionScript)