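; Meteor actor that explodes when its sphere component hits something, breaks into smaller meteors and destroys itself.
; On hit it spawns a giant explosion-radius actor below the sphere and a large explosion particle effect at its location.
; SpawnMeteorSmall spawns small meteors there with random-unit-vector scale, repeating through self-calls and a loop-back capped by a DoN with a random limit.
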(event OnComponentHit(Sphere)
  (params (HitComponent :type Primitive%20Component%20Object%20Reference) (OtherActor :type Actor%20Object%20Reference) (OtherComp :type Primitive%20Component%20Object%20Reference) (NormalImpulse :type Vector :default "0, 0, 0") (Hit :type Hit%20Result%20Structure%20%28by%20ref%29))
  (bind _returnvalue (Transformation|GetWorldLocation HitComponent))
  (Game|SpawnActorfromClass "/Game/Blueprints/ExplosionShotRadiusGiant.ExplosionShotRadiusGiant_C" (Math|Conversions|ToTransform(Vector) (+ _returnvalue "0.000000, 0,-200.000000")) "Undefined" 0 0)
  (CallFunction|SpawnMeteorSmall)
  (Effects|SpawnEmitteratLocation "/Game/StarterContent/Particles/P_Explosion.P_Explosion" _returnvalue "0, 0, 0" "15.000000,15.000000,15.000000")
  (Actor|DestroyActor))

(event Custom|SpawnMeteorSmall
  (Utilities|FlowControl|DoN (Math|Random|RandomIntegerinRange 7 13) :!label _label
    (:Exit
      (Game|SpawnActorfromClass "/Game/Blueprints/Meteor_small.Meteor_small_C" (Math|Transform|MakeTransform (.Location (Math|Transform|BreakTransform (Math|Conversions|ToTransform(Vector) (Transformation|GetWorldLocation (stale OnComponentHit(Sphere) HitComponent))))) (.Rotation (Math|Transform|BreakTransform (Math|Conversions|ToTransform(Vector) (Transformation|GetWorldLocation (stale OnComponentHit(Sphere) HitComponent))))) (Math|Random|RandomUnitVector)) "Undefined" 0 0)
      (CallFunction|SpawnMeteorSmall)
      (goto _label))))

(fn ConstructionScript)