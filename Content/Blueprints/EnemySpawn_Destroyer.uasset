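; Spawner actor that places TowerDestroyerAI enemies at random points inside its SpawnVolume box.
; PickSpawnTime rolls a random delay, and NextSpawn and TimerCheck form a recursive Delay countdown that calls SpawnAI at zero.
; SpawnAI spawns only while SpawnCount is at most one, and each pawn's OnDestroyed lowers the count.
; BeginPlay and Tick are empty, so nothing in this graph starts the loop.
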(event Custom|SpawnAI
  (bind _spawnvolume (Variables|Default|GetSpawnVolume))
  (bind _returnvalue (Components|Box|GetScaledBoxExtent _spawnvolume))
  (bind (_x _y _z) (Math|Vector|BreakVector _returnvalue))
  (if (<= (Variables|Default|GetSpawnCount) 1)
    (bind _returnvalue_2 (AI|SpawnAIFromClass "/Game/GameBPs/Blueprints/TowerDestroyerAI.TowerDestroyerAI_C" 0 (+ (Math|Vector|MakeVector (Math|Random|RandomFloatinRange (* _x -1.0) _x) (Math|Random|RandomFloatinRange (* _y -1.0) _y) (Math|Random|RandomFloatinRange (* _z -1.0) _z)) (Transformation|GetActorLocation)) "0, 0, 0" false))
    (Variables|Default|SetSpawnCount (+ (Variables|Default|GetSpawnCount) 1))
    (for _array_element (Utilities|Array|MakeArray _returnvalue_2)
      (Game|AssignOnDestroyed (stale Custom|Deduct%20Spawn%20Count DestroyedActor) (delegate Custom|Deduct%20Spawn%20Count)))))

(event Custom|NextSpawn
  ;[1 1 1] Countdown Time
  (if (Variables|Default|GetResetTime)
    (Utilities|FlowControl|Delay 1.0)
    (Variables|Default|SetSpawnTimer (- (Variables|Default|GetSpawnTimer) 3.0))
    (CallFunction|NextSpawn)
    (CallFunction|TimerCheck)))

(event Custom|Deduct%20Spawn%20Count
  (params (DestroyedActor :type Actor%20Object%20Reference))
  (Variables|Default|SetSpawnCount (- (Variables|Default|GetSpawnCount) 1)))

(event Custom|TimerCheck
  ;[1 1 1] Time Check
  (if (<= (Variables|Default|GetSpawnTimer) 0.0)
    (Variables|Default|SetResetTime true)
    (Variables|Default|SetCanSpawn? true)
    (CallFunction|PickSpawnTime)
    (CallFunction|SpawnAI)))

(event Custom|PickSpawnTime
  ;[1 1 1] Pick Random Time
  (if (Variables|Default|GetCanSpawn?)
    (Variables|Default|SetSpawnTimer (Math|Random|RandomFloatinRange 15.0 3e+01))
    (CallFunction|NextSpawn)
    (Variables|Default|SetCanSpawn? false)
    (else
      (CallFunction|PickSpawnTime))))

(event EventBeginPlay)

(event EventTick
  (params (DeltaSeconds :type Float%20%28single-precision%29)))

(fn ConstructionScript)