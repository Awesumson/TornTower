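; A test ladder actor that toggles the third-person character's climbing state through a trigger volume.
; Entering ClimbVolume while moving above a small speed threshold sets IsClimbingLadder and passes the ladder's location to the character as LadderPosition.
; Entering while already climbing clears the flag and resets the character to zero world rotation.
; The end-overlap event only casts to the character and takes no action.
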(event OnComponentBeginOverlap(ClimbVolume)
  (params (OverlappedComponent :type Primitive%20Component%20Object%20Reference) (OtherActor :type Actor%20Object%20Reference) (OtherComp :type Primitive%20Component%20Object%20Reference) (OtherBodyIndex :type Integer) (bFromSweep :type Boolean) (SweepResult :type Hit%20Result%20Structure%20%28by%20ref%29))
  (bind _asthird_person_character (Utilities|Casting|CastToThirdPersonCharacter OtherActor))
  (if (Variables|/Game/GameBPs/Blueprints/ThirdPersonCharacter.ThirdPersonCharacter_C|GetIsClimbingLadder _asthird_person_character)
    (Variables|/Game/GameBPs/Blueprints/ThirdPersonCharacter.ThirdPersonCharacter_C|SetIsClimbingLadder _asthird_person_character false)
    (Transformation|SetActorRotation _asthird_person_character)
    (elif (> (Math|Vector|VectorLength (Transformation|GetVelocity _asthird_person_character)) 1e+01)
      (Variables|/Game/GameBPs/Blueprints/ThirdPersonCharacter.ThirdPersonCharacter_C|SetIsClimbingLadder _asthird_person_character true)
      (Variables|/Game/GameBPs/Blueprints/ThirdPersonCharacter.ThirdPersonCharacter_C|SetLadderPosition _asthird_person_character (Transformation|GetActorLocation)))))

(event OnComponentEndOverlap(ClimbVolume)
  (params (OverlappedComponent :type Primitive%20Component%20Object%20Reference) (OtherActor :type Actor%20Object%20Reference) (OtherComp :type Primitive%20Component%20Object%20Reference) (OtherBodyIndex :type Integer))
  (Utilities|Casting|CastToThirdPersonCharacter OtherActor))

(fn ConstructionScript)