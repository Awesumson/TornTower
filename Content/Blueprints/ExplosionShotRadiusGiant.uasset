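; Explosion damage volume, named as the giant shot radius variant, that hurts enemies and mines within its sphere.
; On BeginPlay it spawns an ExplosionSFX actor at its location.
; Any sphere overlap sets a one-second lifespan, so removal is only scheduled once something overlaps.
; Overlapping actors tagged Enemy or Mine trigger fixed damage, applied to the sweep result's hit actor rather than the overlapping actor.
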(event OnComponentBeginOverlap(Sphere)
  (params (OverlappedComponent :type Primitive%20Component%20Object%20Reference) (OtherActor :type Actor%20Object%20Reference) (OtherComp :type Primitive%20Component%20Object%20Reference) (OtherBodyIndex :type Integer) (bFromSweep :type Boolean) (SweepResult :type Hit%20Result%20Structure%20%28by%20ref%29))
  (Actor|SetLifeSpan 1.0)
  (if (Actor|ActorHasTag OtherActor "Enemy")
    (Game|Damage|ApplyDamage (.HitActor (Collision|BreakHitResult SweepResult)) 5e+01 0 0 :!label _label)
    (elif (Actor|ActorHasTag OtherActor "Mine")
      (goto _label))))

(event EventBeginPlay
  (Game|SpawnActorfromClass "/Game/ExplosionSFX.ExplosionSFX_C" (Math|Conversions|ToTransform(Vector) (Transformation|GetActorLocation)) "Undefined" 0 0))

(fn ConstructionScript)