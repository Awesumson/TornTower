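; Airstrike spawner actor that scatters a burst of AirstrikeRadius actors across an area when play begins.
; Each spawn lands at a random point within the SpawnVolume box's scaled extents, offset from the actor's location without applying its rotation.
; A short Delay and a DoN node loop back to the spawn step, producing eleven staggered spawns in total.
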(event Collision|EventActorBeginOverlap
  (params (OtherActor :type Actor%20Object%20Reference)))

(event EventTick
  (params (DeltaSeconds :type Float%20%28single-precision%29)))

(event EventBeginPlay
  (bind _spawn_volume (Variables|Default|GetSpawn%20Volume))
  (bind _returnvalue (Components|Box|GetScaledBoxExtent _spawn_volume))
  (bind (_x _y _z) (Math|Vector|BreakVector _returnvalue))
  (Game|SpawnActorfromClass "/Game/Blueprints/AirstrikeRadius.AirstrikeRadius_C" (Math|Conversions|ToTransform(Vector) (+ (Math|Vector|MakeVector (Math|Random|RandomFloatinRange (* _x -1.0) _x) (Math|Random|RandomFloatinRange (* _y -1.0) _y) (Math|Random|RandomFloatinRange (* _z -1.0) _z)) (Transformation|GetActorLocation))) "Undefined" 0 0 :!label _label)
  (Utilities|FlowControl|Delay 0.2)
  (Utilities|FlowControl|DoN 10
    (:Exit
      (goto _label))))

(fn ConstructionScript)