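; EnergyBoxSmall is an energy pickup actor that expires 30 seconds after it spawns.
; When a ThirdPersonCharacterTT overlaps it, it raises that character's TotalEnergy by a fixed amount capped at the maximum, then destroys itself.
; If energy was added and no popup is showing, it sets the popup flag, calls ResetPopup and shows an EnergyCollected widget.
; A character already at full energy still consumes the box.
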(event Collision|EventActorBeginOverlap
  (params (OtherActor :type Actor%20Object%20Reference))
  (bind _asthird_person_character_tt (Utilities|Casting|CastToThirdPersonCharacterTT OtherActor))
  (if (>= (Variables|/Game/GameBPs/Blueprints/ThirdPersonCharacterTT.ThirdPersonCharacterTT_C|GetTotalEnergy _asthird_person_character_tt) 1e+02)
    (Actor|DestroyActor)
    (else
      (if (>= (Variables|/Game/GameBPs/Blueprints/ThirdPersonCharacterTT.ThirdPersonCharacterTT_C|GetTotalEnergy _asthird_person_character_tt) 5e+01)
        (Variables|/Game/GameBPs/Blueprints/ThirdPersonCharacterTT.ThirdPersonCharacterTT_C|SetTotalEnergy _asthird_person_character_tt 1e+02)
        (else
          (Variables|/Game/GameBPs/Blueprints/ThirdPersonCharacterTT.ThirdPersonCharacterTT_C|SetTotalEnergy _asthird_person_character_tt (+ (Variables|/Game/GameBPs/Blueprints/ThirdPersonCharacterTT.ThirdPersonCharacterTT_C|GetTotalEnergy _asthird_person_character_tt) 5e+01))))
      (Actor|DestroyActor)
      (if (not (Variables|/Game/GameBPs/Blueprints/ThirdPersonCharacterTT.ThirdPersonCharacterTT_C|GetPopupDisplayed? _asthird_person_character_tt))
        (Variables|/Game/GameBPs/Blueprints/ThirdPersonCharacterTT.ThirdPersonCharacterTT_C|SetPopupDisplayed? _asthird_person_character_tt true)
        (Default|ResetPopup _asthird_person_character_tt)
        (bind _returnvalue (UserInterface|CreateWidget "/Game/Interfaces/EnergyCollected.EnergyCollected_C" (Game|GetPlayerController 0)))
        (UserInterface|Viewport|AddtoViewport _returnvalue 0)))))

(event EventBeginPlay
  (Actor|SetLifeSpan 3e+01))

(fn ConstructionScript)