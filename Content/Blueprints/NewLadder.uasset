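; NewLadder is a ladder actor whose Box volume lets the ThirdPersonCharacterTT climb by switching its movement mode.
; On begin overlap, it casts the overlapping actor, sets movement to Flying and constrains the movement primitive to the YZ plane.
; End overlap restores Walking on that cast character without checking which actor left or resetting the constraint.
; The constraint reset sits in an else branch that never runs, since InLadderVolume is set true just before the check.
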(event OnComponentBeginOverlap(Box)
  (params (OverlappedComponent :type Primitive%20Component%20Object%20Reference) (OtherActor :type Actor%20Object%20Reference) (OtherComp :type Primitive%20Component%20Object%20Reference) (OtherBodyIndex :type Integer) (bFromSweep :type Boolean) (SweepResult :type Hit%20Result%20Structure%20%28by%20ref%29))
  (Variables|Default|SetInLadderVolume? true)
  (bind _asthird_person_character_tt (Utilities|Casting|CastToThirdPersonCharacterTT OtherActor))
  (if (Variables|Default|GetInLadderVolume?)
    (Pawn|Components|CharacterMovement|SetMovementMode (Variables|/Script/Engine.Character|GetCharacterMovement _asthird_person_character_tt) "MOVE_Flying" 0)
    (Class|PrimitiveComponent|SetConstraintMode (Variables|/Script/Engine.MovementComponent|GetUpdatedPrimitive (Variables|/Script/Engine.Character|GetCharacterMovement _asthird_person_character_tt)) "YZPlane")
    (else
      (Pawn|Components|CharacterMovement|SetMovementMode (Variables|/Script/Engine.Character|GetCharacterMovement _asthird_person_character_tt) "MOVE_Walking" 0)
      (Class|PrimitiveComponent|SetConstraintMode (Variables|/Script/Engine.MovementComponent|GetUpdatedPrimitive (Variables|/Script/Engine.Character|GetCharacterMovement _asthird_person_character_tt)) "Default"))))

(event OnComponentEndOverlap(Box)
  (params (OverlappedComponent :type Primitive%20Component%20Object%20Reference) (OtherActor :type Actor%20Object%20Reference) (OtherComp :type Primitive%20Component%20Object%20Reference) (OtherBodyIndex :type Integer))
  (Variables|Default|SetInLadderVolume? false)
  (Pawn|Components|CharacterMovement|SetMovementMode (Variables|/Script/Engine.Character|GetCharacterMovement (stale OnComponentBeginOverlap(Box) _asthird_person_character_tt)) "MOVE_Walking" 0))

(fn ConstructionScript)