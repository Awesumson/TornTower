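; Enemy spawner actor that places a laser or cannon Stalker AI at a random point inside its SpawnVolume box.
; Self-calling events form a one-second countdown from a random interval, then re-roll it and attempt a spawn.
; Spawning requires a zero SpawnCount, which rises on each spawn and is meant to fall through OnDestroyed bindings.
; BeginPlay is empty, so nothing in this graph starts the cycle.
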(event Custom|SpawnAI
  (bind _returnvalue (Transformation|GetActorLocation))
  (bind _spawnvolume (Variables|Default|GetSpawnVolume))
  (bind _returnvalue_2 (Components|Box|GetScaledBoxExtent _spawnvolume))
  (bind (_x _y _z) (Math|Vector|BreakVector _returnvalue_2))
  (bind _returnvalue_3 (* _z -1.0))
  (bind _returnvalue_4 (* _x -1.0))
  (bind _returnvalue_5 (* _y -1.0))
  (bind _returnvalue_6 (Math|Random|RandomFloatinRange _returnvalue_3 _z))
  (bind _returnvalue_7 (Math|Random|RandomFloatinRange _returnvalue_4 _x))
  (bind _returnvalue_8 (Math|Random|RandomFloatinRange _returnvalue_5 _y))
  (bind _returnvalue_9 (Math|Vector|MakeVector _returnvalue_7 _returnvalue_8 _returnvalue_6))
  (bind _returnvalue_10 (+ _returnvalue_9 _returnvalue))
  (if (== (Variables|Default|GetSpawnCount) 0)
    (switch int (Math|Random|RandomIntegerinRange 0 1)
      (:0
        (bind _returnvalue_11 (AI|SpawnAIFromClass "/Game/GameBPs/Blueprints/StalkerAI_laser.StalkerAI_laser_C" 0 _returnvalue_10 "0, 0, 0" false)))
      (:1
        (bind _returnvalue_12 (AI|SpawnAIFromClass "/Game/GameBPs/Blueprints/StalkerAI_cannon.StalkerAI_cannon_C" 0 _returnvalue_10 "0, 0, 0" false))))
    (Variables|Default|SetSpawnCount (+ (Variables|Default|GetSpawnCount) 1))
    (for _array_element (Utilities|Array|MakeArray _returnvalue_12)
      (for _array_element_2 (Utilities|Array|MakeArray _returnvalue_11)
        (Game|AssignOnDestroyed (stale Custom|Deduct%20Spawn%20Count DestroyedActor) (delegate Custom|Deduct%20Spawn%20Count))))))

(event Custom|NextSpawn
  ;[1 1 1] Countdown Time
  (if (Variables|Default|GetResetTime)
    (Utilities|FlowControl|Delay 1.0)
    (Variables|Default|SetSpawnTimer (- (Variables|Default|GetSpawnTimer) 1.0))
    (CallFunction|NextSpawn)
    (CallFunction|TimerCheck)))

(event Custom|Deduct%20Spawn%20Count
  (params (DestroyedActor :type Actor%20Object%20Reference))
  (Variables|Default|SetSpawnCount (- (Variables|Default|GetSpawnCount) 1)))

(event Custom|TimerCheck
  ;[1 1 1] Time Check
  (if (<= (Variables|Default|GetSpawnTimer) 0.0)
    (Variables|Default|SetResetTime true)
    (Variables|Default|SetCanSpawn? true)
    (CallFunction|PickSpawnTime)
    (CallFunction|SpawnAI)))

(event Custom|PickSpawnTime
  ;[1 1 1] Pick Random Time
  (if (Variables|Default|GetCanSpawn?)
    (Variables|Default|SetSpawnTimer (Math|Random|RandomFloatinRange 3e+01 5e+01))
    (CallFunction|NextSpawn)
    (Variables|Default|SetCanSpawn? false)
    (else
      (CallFunction|PickSpawnTime))))

(event EventBeginPlay)

(event EventTick
  (params (DeltaSeconds :type Float%20%28single-precision%29)))

(fn ConstructionScript)