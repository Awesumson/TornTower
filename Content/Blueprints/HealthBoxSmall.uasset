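; HealthBoxSmall is a small health pickup that expires after a limited lifespan set on BeginPlay.
; When a ThirdPersonCharacterTT overlaps it, it adds one to that character's TotalHealth and destroys itself.
; It then shows a HealthCollectedSmall widget for player 0, using the character's PopupDisplayed flag and ResetPopup call to avoid stacking popups.
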(event Collision|EventActorBeginOverlap
  (params (OtherActor :type Actor%20Object%20Reference))
  (bind _asthird_person_character_tt (Utilities|Casting|CastToThirdPersonCharacterTT OtherActor))
  (Variables|/Game/GameBPs/Blueprints/ThirdPersonCharacterTT.ThirdPersonCharacterTT_C|SetTotalHealth _asthird_person_character_tt (+ (Variables|/Game/GameBPs/Blueprints/ThirdPersonCharacterTT.ThirdPersonCharacterTT_C|GetTotalHealth _asthird_person_character_tt) 1))
  (Actor|DestroyActor)
  (if (not (Variables|/Game/GameBPs/Blueprints/ThirdPersonCharacterTT.ThirdPersonCharacterTT_C|GetPopupDisplayed? _asthird_person_character_tt))
    (Variables|/Game/GameBPs/Blueprints/ThirdPersonCharacterTT.ThirdPersonCharacterTT_C|SetPopupDisplayed? _asthird_person_character_tt true)
    (Default|ResetPopup _asthird_person_character_tt)
    (bind _returnvalue (UserInterface|CreateWidget "/Game/Interfaces/HealthCollectedSmall.HealthCollectedSmall_C" (Game|GetPlayerController 0)))
    (UserInterface|Viewport|AddtoViewport _returnvalue 0)))

(event EventBeginPlay
  (Actor|SetLifeSpan 3e+01))

(fn ConstructionScript)