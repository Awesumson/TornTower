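; TowerRepairKit is a pickup that restores a random amount of tower health when the third-person character overlaps it.
; BeginPlay rolls the amount; overlap records it on the first TowerHP actor found, adding it only below the health threshold, without clamping.
; If no popup is displayed, it flags the character's popup, calls ResetPopup, shows the TowerRepairCollected widget and destroys itself.
; Otherwise the kit remains in the world.
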(event Custom|Set%20Health%20Addition)

(event Collision|EventActorBeginOverlap
  (params (OtherActor :type Actor%20Object%20Reference))
  (bind _asthird_person_character_tt (Utilities|Casting|CastToThirdPersonCharacterTT OtherActor))
  (bind _outactors (Actor|GetAllActorsOfClass "/Game/Blueprints/TowerHP.TowerHP_C"))
  (bind _astower_hp (Utilities|Casting|CastToTowerHP (Utilities|Array|Get(acopy) _outactors)))
  (Variables|/Game/Blueprints/TowerHP.TowerHP_C|SetLast%20Health%20Addition _astower_hp (Variables|Default|GetRepairAmount))
  (if (< (Variables|/Game/Blueprints/TowerHP.TowerHP_C|GetTowerHealth _astower_hp) 1500)
    (Variables|/Game/Blueprints/TowerHP.TowerHP_C|SetTowerHealth _astower_hp (+ (Variables|/Game/Blueprints/TowerHP.TowerHP_C|GetTowerHealth _astower_hp) (Variables|Default|GetRepairAmount)))
    (if (not (Variables|/Game/GameBPs/Blueprints/ThirdPersonCharacterTT.ThirdPersonCharacterTT_C|GetPopupDisplayed? _asthird_person_character_tt))
      (Variables|/Game/GameBPs/Blueprints/ThirdPersonCharacterTT.ThirdPersonCharacterTT_C|SetPopupDisplayed? _asthird_person_character_tt true)
      (Default|ResetPopup _asthird_person_character_tt)
      (bind _returnvalue (UserInterface|CreateWidget "/Game/Interfaces/TowerRepairCollected.TowerRepairCollected_C" (Game|GetPlayerController 0)))
      (UserInterface|Viewport|AddtoViewport _returnvalue 0)
      (Actor|DestroyActor))))

(event EventBeginPlay
  (Variables|Default|SetRepairAmount (Math|Random|RandomIntegerinRange 35 115))
  (Utilities|FlowControl|Delay 0.2))

(fn ConstructionScript)