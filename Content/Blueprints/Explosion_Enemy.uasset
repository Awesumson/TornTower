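; Explosion_Enemy is an explosion actor that damages whatever overlaps it, with an extra health penalty for the third-person character.
; BeginPlay draws a brief debug sphere at its location and spawns an ExplosionSFX actor there.
; Each overlap sets a short lifespan and applies damage to the other actor, then directly subtracts from TotalHealth if that actor is a ThirdPersonCharacterTT.
; The lifespan is set only on overlap.
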(event Collision|EventActorBeginOverlap
  (params (OtherActor :type Actor%20Object%20Reference))
  (Actor|SetLifeSpan 1.0)
  (Game|Damage|ApplyDamage OtherActor 3e+02 0 0)
  (bind _asthird_person_character_tt (Utilities|Casting|CastToThirdPersonCharacterTT OtherActor))
  (Variables|/Game/GameBPs/Blueprints/ThirdPersonCharacterTT.ThirdPersonCharacterTT_C|SetTotalHealth _asthird_person_character_tt (- (Variables|/Game/GameBPs/Blueprints/ThirdPersonCharacterTT.ThirdPersonCharacterTT_C|GetTotalHealth _asthird_person_character_tt) 3)))

(event EventBeginPlay
  (bind _returnvalue (Transformation|GetActorLocation))
  (Rendering|Debug|DrawDebugSphere _returnvalue 3e+02 12 "(R=1.000000,G=0.000000,B=0.009094,A=1.000000)" 1.0 2.0)
  (Game|SpawnActorfromClass "/Game/ExplosionSFX.ExplosionSFX_C" (Math|Conversions|ToTransform(Vector) _returnvalue) "Undefined" 0 0))

(fn ConstructionScript)