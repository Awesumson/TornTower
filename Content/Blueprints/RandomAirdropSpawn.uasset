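; RandomAirdropSpawn is an actor that repeatedly spawns random airdrop pickups: health, energy, damage amp, ammo variants and care packages.
; PickSpawnTime sets a short random timer, which NextSpawn counts down through a self-calling Delay loop gated by ResetTime.
; When TimerCheck sees it expire, it re-arms the timer and calls SpawnAmmo.
; SpawnAmmo places one random class within the SpawnVolume extents around the actor and sets a limited lifespan.
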(event Custom|Spawn%20Ammo
  (bind _returnvalue (Transformation|GetActorLocation))
  (bind _spawnvolume (Variables|Default|GetSpawnVolume))
  (bind _returnvalue_2 (Components|Box|GetScaledBoxExtent _spawnvolume))
  (bind (_x _y _z) (Math|Vector|BreakVector _returnvalue_2))
  (bind _returnvalue_3 (* _z -1.0))
  (bind _returnvalue_4 (* _x -1.0))
  (bind _returnvalue_5 (* _y -1.0))
  (bind _returnvalue_6 (Math|Random|RandomFloatinRange _returnvalue_3 _z))
  (bind _returnvalue_7 (Math|Random|RandomFloatinRange _returnvalue_4 _x))
  (bind _returnvalue_8 (Math|Random|RandomFloatinRange _returnvalue_5 _y))
  (bind _returnvalue_9 (Math|Vector|MakeVector _returnvalue_7 _returnvalue_8 _returnvalue_6))
  (bind _returnvalue_10 (+ _returnvalue_9 _returnvalue))
  (bind _returnvalue_11 (Math|Transform|MakeTransform _returnvalue_10))
  (switch int (Math|Random|RandomIntegerinRange 0 7)
    (:0
      (bind _returnvalue_12 (Game|SpawnActorfromClass "/Game/Blueprints/HealthBox.HealthBox_C" _returnvalue_11 "Undefined" 0 0)))
    (:1
      (bind _returnvalue_13 (Game|SpawnActorfromClass "/Game/Blueprints/AmmoBox.AmmoBox_C" _returnvalue_11 "Undefined" 0 0)))
    (:2
      (bind _returnvalue_14 (Game|SpawnActorfromClass "/Game/Blueprints/EnergyBox.EnergyBox_C" _returnvalue_11 "Undefined" 0 0)))
    (:3
      (bind _returnvalue_15 (Game|SpawnActorfromClass "/Game/Blueprints/AMPDamageBox.AMPDamageBox_C" _returnvalue_11 "Undefined" 0 0)))
    (:4
      (bind _returnvalue_16 (Game|SpawnActorfromClass "/Game/Blueprints/CryoAmmoBox.CryoAmmoBox_C" _returnvalue_11 "Undefined" 0 0)))
    (:5
      (bind _returnvalue_17 (Game|SpawnActorfromClass "/Game/Blueprints/AmmoRegenBox.AmmoRegenBox_C" _returnvalue_11 "Undefined" 0 0)))
    (:6
      (bind _returnvalue_18 (Game|SpawnActorfromClass "/Game/Blueprints/CarePackage.CarePackage_C" _returnvalue_11 "Undefined" 0 0)))
    (:7
      (bind _returnvalue_19 (Game|SpawnActorfromClass "/Game/Blueprints/ExplosiveAmmoBox.ExplosiveAmmoBox_C" _returnvalue_11 "Undefined" 0 0))))
  (Actor|SetLifeSpan _returnvalue_12 1.2e+02) ; Ammo Box Life Span
)

(event Custom|NextSpawn
  ;[1 1 1] Countdown Time
  (if (Variables|Default|GetResetTime)
    (Utilities|FlowControl|Delay 1.0)
    (Variables|Default|SetSpawnTimer (- (Variables|Default|GetSpawnTimer) 1.0))
    (CallFunction|NextSpawn)
    (CallFunction|TimerCheck)))

(event Custom|TimerCheck
  ;[1 1 1] Time Check
  (if (<= (Variables|Default|GetSpawnTimer) 0.0)
    (Variables|Default|SetResetTime true)
    (Variables|Default|SetCanSpawn? true)
    (CallFunction|PickSpawnTime)
    (CallFunction|SpawnAmmo)))

(event Custom|PickSpawnTime
  ;[1 1 1] Pick Random Time
  (if (Variables|Default|GetCanSpawn?)
    (Variables|Default|SetSpawnTimer (Math|Random|RandomFloatinRange 0.5 1.0))
    (CallFunction|NextSpawn)
    (Variables|Default|SetCanSpawn? false)
    (else
      (CallFunction|PickSpawnTime))))

(event EventBeginPlay
  (CallFunction|PickSpawnTime))

(event EventTick
  (params (DeltaSeconds :type Float%20%28single-precision%29)))

(fn ConstructionScript)