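; Enemy AI character that seeks out and attacks the TowerHP actor, ignoring players.
; Every Tick it checks health and re-issues AIMoveTo; overlapping the tower starts a self-repeating, delayed damage loop that never clears.
; At zero health it awards score to the first ThirdPersonCharacter and drops a random ammo pickup, weighted toward small boxes.
; Cryo projectile hits temporarily slow it and tint it cyan; MassFreeze applies a longer slow.
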(event Custom|DamageTower
  ;[1 1 1] DamageTower
  (if (Variables|Default|GetInAttackRange)
    (Utilities|FlowControl|Delay 1.0)
    (bind _outactors (Actor|GetAllActorsOfClass "/Game/Blueprints/TowerHP.TowerHP_C"))
    (Default|TakeDamage (Utilities|Array|Get(acopy) _outactors))
    (else
      (Utilities|FlowControl|Delay 1.0)))
  (CallFunction|DamageTower))

(event Custom|Update%20Score
  (bind _outactors (Actor|GetAllActorsOfClass "/Game/GameBPs/Blueprints/ThirdPersonCharacter.ThirdPersonCharacter_C"))
  (bind _asthird_person_character (Utilities|Casting|CastToThirdPersonCharacter (Utilities|Array|Get(acopy) _outactors)))
  (Variables|/Game/GameBPs/Blueprints/ThirdPersonCharacter.ThirdPersonCharacter_C|SetScore _asthird_person_character (+ (Variables|/Game/GameBPs/Blueprints/ThirdPersonCharacter.ThirdPersonCharacter_C|GetScore _asthird_person_character) 100)))

(event Custom|MassFreeze
  ;[0 1 0.9624] MassFreeze
  (Variables|/Script/Engine.CharacterMovementComponent|SetMaxWalkSpeed (Variables|Character|GetCharacterMovement) 1e+02)
  (Utilities|FlowControl|Delay 15.0)
  (Variables|/Script/Engine.CharacterMovementComponent|SetMaxWalkSpeed (Variables|Character|GetCharacterMovement) 2e+02))

(event Custom|Advance%20towards%20player
  (CallFunction|HealthCheck)
  (bind _outactors (Actor|GetAllActorsOfClass "/Game/Blueprints/TowerHP.TowerHP_C"))
  (AI|AIMoveTo self "0, 0, 0" (Utilities|Array|Get(acopy) _outactors) (Variables|Default|GetRange) false))

(event Custom|Health%20Check
  (bind _returnvalue (Transformation|GetActorLocation))
  (bind _returnvalue_2 (Math|Conversions|ToTransform(Vector) _returnvalue))
  (if (<= (Variables|Default|GetHealth) 0.0)
    (CallFunction|UpdateScore)
    (Actor|DestroyActor)
    (switch int (Math|Random|RandomIntegerinRange 0 3)
      (:0
        (Game|SpawnActorfromClass "/Game/Blueprints/AmmoBoxSmall.AmmoBoxSmall_C" _returnvalue_2 "Undefined" 0 0 :!label _label))
      (:1
        (goto _label))
      (:2
        (Game|SpawnActorfromClass "/Game/Blueprints/AmmoBox.AmmoBox_C" _returnvalue_2 "Undefined" 0 0))
      (:3
        (Game|SpawnActorfromClass "/Game/Blueprints/AmmoRegenBox.AmmoRegenBox_C" _returnvalue_2 "Undefined" 0 0)))))

(event EventBeginPlay
  (CallFunction|AdvanceTowardsPlayer))

(event Collision|EventActorEndOverlap
  (params (OtherActor :type Actor%20Object%20Reference))
  ;[1 1 1] DamageTower
)

(event Collision|EventActorBeginOverlap
  (params (OtherActor :type Actor%20Object%20Reference))
  ;[1 1 1] DamageTower
  (Utilities|Casting|CastToTowerHP OtherActor)
  (Variables|Default|SetInAttackRange true)
  (CallFunction|DamageTower))

(event EventTick
  (params (DeltaSeconds :type Float%20%28single-precision%29))
  (CallFunction|AdvanceTowardsPlayer))

(event Game|Damage|EventAnyDamage
  (params (Damage :type Float%20%28single-precision%29) (DamageType :type Damage%20Type%20Object%20Reference) (InstigatedBy :type Controller%20Object%20Reference) (DamageCauser :type Actor%20Object%20Reference))
  (Variables|Default|SetHealth (- (Variables|Default|GetHealth) Damage)))

(event Collision|EventHit
  (params (MyComp :type Primitive%20Component%20Object%20Reference) (Other :type Actor%20Object%20Reference) (OtherComp :type Primitive%20Component%20Object%20Reference) (bSelfMoved :type Boolean) (HitLocation :type Vector :default "0, 0, 0") (HitNormal :type Vector :default "0, 0, 0") (NormalImpulse :type Vector :default "0, 0, 0") (Hit :type Hit%20Result%20Structure%20%28by%20ref%29))
  (bind _mesh (Variables|Character|GetMesh))
  (bind _charactermovement (Variables|Character|GetCharacterMovement))
  (bind _mesh_2 (Variables|Character|GetMesh))
  (Utilities|Casting|CastToCryoProjectileNEW Other)
  (Variables|/Script/Engine.CharacterMovementComponent|SetMaxWalkSpeed _charactermovement 1e+02)
  (Rendering|Material|SetMaterial _mesh_2 0 "/Game/Wireframe_2_M_Cyan.Wireframe_2_M_Cyan")
  (Rendering|Material|SetMaterial _mesh_2 1 "/Game/Wireframe_2_M_Cyan.Wireframe_2_M_Cyan")
  (Utilities|FlowControl|Delay 1e+01)
  (Variables|/Script/Engine.CharacterMovementComponent|SetMaxWalkSpeed _charactermovement 2e+02)
  (Rendering|Material|SetMaterial _mesh 0 "/Game/Wireframe_2_M.Wireframe_2_M")
  (Rendering|Material|SetMaterial _mesh 1 "/Game/Wireframe_2_M.Wireframe_2_M"))

(fn ConstructionScript)