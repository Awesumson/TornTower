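; Suicide bomber enemy AI that chases the first player, then stops within close range and explodes after a short delay.
; Every Tick re-issues the move order and runs range and health checks.
; Damage lowers health; death adds score to the player character and may drop a small ammo, health or energy box.
; Cryo projectile hits and the MassFreeze event temporarily slow it and tint its mesh cyan.
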(event Custom|Update%20Score
  (bind _outactors (Actor|GetAllActorsOfClass "/Game/GameBPs/Blueprints/ThirdPersonCharacterTT.ThirdPersonCharacterTT_C"))
  (bind _asthird_person_character_tt (Utilities|Casting|CastToThirdPersonCharacterTT (Utilities|Array|Get(acopy) _outactors)))
  (Variables|/Game/GameBPs/Blueprints/ThirdPersonCharacterTT.ThirdPersonCharacterTT_C|SetScore _asthird_person_character_tt (+ 200 (Variables|/Game/GameBPs/Blueprints/ThirdPersonCharacterTT.ThirdPersonCharacterTT_C|GetScore _asthird_person_character_tt))))

(event Custom|RangeFinder
  ;[1 1 1] Attack Range
  (if (<= (Math|Vector|VectorLength (- (Transformation|GetActorLocation (Game|Player|GetPlayerPawn 0)) (Transformation|GetActorLocation))) 3e+02)
    (Variables|Default|SetInAttackRange true)
    (if (Variables|Default|GetInAttackRange)
      (Pawn|Components|CharacterMovement|DisableMovement (Variables|Character|GetCharacterMovement))
      (Utilities|FlowControl|Delay 0.5)
      (Game|SpawnActorfromClass "/Game/Blueprints/Explosion_Enemy.Explosion_Enemy_C" (Math|Conversions|ToTransform(Vector) (Transformation|GetActorLocation)) "Undefined" 0 0)
      (Effects|SpawnEmitteratLocation "/Game/StarterContent/Particles/P_Explosion.P_Explosion" (Transformation|GetActorLocation) "0, 0, 0" "7.000000,7.000000,7.000000" false)
      (Actor|DestroyActor))))

(event Custom|MassFreeze
  (bind _mesh (Variables|Character|GetMesh))
  (bind _mesh_2 (Variables|Character|GetMesh))
  ;[0 1 0.9624] MassFreeze
  (Variables|/Script/Engine.CharacterMovementComponent|SetMaxWalkSpeed (Variables|Character|GetCharacterMovement) 1.5e+02)
  (Rendering|Material|SetMaterial _mesh 1 "/Game/Wireframe_2_M_Cyan.Wireframe_2_M_Cyan")
  (Rendering|Material|SetMaterial _mesh 0 "/Game/Wireframe_2_M_Cyan.Wireframe_2_M_Cyan")
  (Utilities|FlowControl|Delay 15.0)
  (Variables|/Script/Engine.CharacterMovementComponent|SetMaxWalkSpeed (Variables|Character|GetCharacterMovement) 5e+02)
  (Rendering|Material|SetMaterial _mesh_2 0 "/Game/Wireframe_2_M.Wireframe_2_M")
  (Rendering|Material|SetMaterial _mesh_2 1 "/Game/Wireframe_2_M.Wireframe_2_M"))

(event Custom|Advance%20towards%20player
  (CallFunction|RangeFinder)
  (CallFunction|HealthCheck)
  (AI|AIMoveTo self "0, 0, 0" (Game|GetPlayerCharacter 0) (Variables|Default|GetRange) false))

(event Custom|Health%20Check
  (bind _returnvalue (Transformation|GetActorLocation))
  (bind _returnvalue_2 (Math|Conversions|ToTransform(Vector) _returnvalue))
  (if (<= (Variables|Default|GetHealth) 0.0)
    (CallFunction|UpdateScore)
    (Actor|DestroyActor)
    (switch int (Math|Random|RandomIntegerinRange 0 9)
      (:0
        (Game|SpawnActorfromClass "/Game/Blueprints/AmmoBoxSmall.AmmoBoxSmall_C" _returnvalue_2 "Undefined" 0 0))
      (:1
        (Game|SpawnActorfromClass "/Game/Blueprints/HealthBoxSmall.HealthBoxSmall_C" _returnvalue_2 "Undefined" 0 0))
      (:2
        (Game|SpawnActorfromClass "/Game/Blueprints/EnergyBoxSmall.EnergyBoxSmall_C" _returnvalue_2 "Undefined" 0 0)))))

(event EventBeginPlay
  (CallFunction|AdvanceTowardsPlayer))

(event EventTick
  (params (DeltaSeconds :type Float%20%28single-precision%29))
  (CallFunction|AdvanceTowardsPlayer))

(event Game|Damage|EventAnyDamage
  (params (Damage :type Float%20%28single-precision%29) (DamageType :type Damage%20Type%20Object%20Reference) (InstigatedBy :type Controller%20Object%20Reference) (DamageCauser :type Actor%20Object%20Reference))
  (Variables|Default|SetHealth (- (Variables|Default|GetHealth) Damage)))

(event Collision|EventHit
  (params (MyComp :type Primitive%20Component%20Object%20Reference) (Other :type Actor%20Object%20Reference) (OtherComp :type Primitive%20Component%20Object%20Reference) (bSelfMoved :type Boolean) (HitLocation :type Vector :default "0, 0, 0") (HitNormal :type Vector :default "0, 0, 0") (NormalImpulse :type Vector :default "0, 0, 0") (Hit :type Hit%20Result%20Structure%20%28by%20ref%29))
  (bind _mesh (Variables|Character|GetMesh))
  (bind _charactermovement (Variables|Character|GetCharacterMovement))
  (bind _mesh_2 (Variables|Character|GetMesh))
  (Utilities|Casting|CastToCryoProjectileNEW Other)
  (Variables|/Script/Engine.CharacterMovementComponent|SetMaxWalkSpeed _charactermovement 1.5e+02)
  (Rendering|Material|SetMaterial _mesh_2 0 "/Game/Wireframe_2_M_Cyan.Wireframe_2_M_Cyan")
  (Rendering|Material|SetMaterial _mesh_2 1 "/Game/Wireframe_2_M_Cyan.Wireframe_2_M_Cyan")
  (Utilities|FlowControl|Delay 1e+01)
  (Variables|/Script/Engine.CharacterMovementComponent|SetMaxWalkSpeed _charactermovement 9e+02)
  (Rendering|Material|SetMaterial _mesh 0 "/Game/Wireframe_2_M.Wireframe_2_M")
  (Rendering|Material|SetMaterial _mesh 1 "/Game/Wireframe_2_M.Wireframe_2_M"))

(fn ConstructionScript)