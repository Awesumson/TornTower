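; Basic enemy AI character that chases the first player and attacks at close range.
; Every tick it checks range, checks health and re-issues AIMoveTo; cooldown-gated attacks hit the player or the Stalker vehicle they occupy.
; Damage and headshot events lower health, while cryo hits and MassFreeze temporarily slow it and tint it cyan.
; Headshots and death add score, and death destroys it with a random chance of an ammo, health or energy pickup.
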(event Custom|HeadHit
  (Variables|Default|SetHealth (- (Variables|Default|GetHealth) 1e+02))
  (bind _outactors (Actor|GetAllActorsOfClass "/Game/GameBPs/Blueprints/ThirdPersonCharacterTT.ThirdPersonCharacterTT_C"))
  (bind _asthird_person_character_tt (Utilities|Casting|CastToThirdPersonCharacterTT (Utilities|Array|Get(acopy) _outactors)))
  (Variables|/Game/GameBPs/Blueprints/ThirdPersonCharacterTT.ThirdPersonCharacterTT_C|SetScore _asthird_person_character_tt (+ (Variables|/Game/GameBPs/Blueprints/ThirdPersonCharacterTT.ThirdPersonCharacterTT_C|GetScore _asthird_person_character_tt) 1)))

(event Custom|AttackPlayer
  ;[1 1 1] Attack
  (if (Variables|Default|GetInAttackRange)
    (if (Variables|Default|GetCanAttack)
      (bind _outactors (Actor|GetAllActorsOfClass "/Game/GameBPs/Blueprints/ThirdPersonCharacterTT.ThirdPersonCharacterTT_C"))
      (bind _asthird_person_character_tt (Utilities|Casting|CastToThirdPersonCharacterTT (Utilities|Array|Get(acopy) _outactors)))
      (if (or (Variables|/Game/GameBPs/Blueprints/ThirdPersonCharacterTT.ThirdPersonCharacterTT_C|GetInVehicle_1 _asthird_person_character_tt) (Variables|/Game/GameBPs/Blueprints/ThirdPersonCharacterTT.ThirdPersonCharacterTT_C|GetInVehicle_2 _asthird_person_character_tt))
        (if (Variables|/Game/GameBPs/Blueprints/ThirdPersonCharacterTT.ThirdPersonCharacterTT_C|GetInVehicle_1 _asthird_person_character_tt)
          (bind _outactors_2 (Actor|GetAllActorsOfClass "/Game/GameBPs/Blueprints/StalkerAI_auto_controllable.StalkerAI_auto_controllable_C"))
          (bind _asstalker_ai_auto_controllable (Utilities|Casting|CastToStalkerAI_auto_controllable (Utilities|Array|Get(acopy) _outactors_2)))
          (Variables|/Game/GameBPs/Blueprints/StalkerAI_auto_controllable.StalkerAI_auto_controllable_C|SetHealth _asstalker_ai_auto_controllable (- (Variables|/Game/GameBPs/Blueprints/StalkerAI_auto_controllable.StalkerAI_auto_controllable_C|GetHealth _asstalker_ai_auto_controllable) 2e+01))
          (Variables|Default|SetCanAttack false :!label _label)
          (CallFunction|AttackDelay)
          (elif (Variables|/Game/GameBPs/Blueprints/ThirdPersonCharacterTT.ThirdPersonCharacterTT_C|GetInVehicle_2 _asthird_person_character_tt)
            (bind _outactors_3 (Actor|GetAllActorsOfClass "/Game/GameBPs/Blueprints/StalkerAI_fullcontrollable.StalkerAI_fullcontrollable_C"))
            (bind _asstalker_ai_fullcontrollable (Utilities|Casting|CastToStalkerAI_fullcontrollable (Utilities|Array|Get(acopy) _outactors_3)))
            (Variables|/Game/GameBPs/Blueprints/StalkerAI_fullcontrollable.StalkerAI_fullcontrollable_C|SetHealth _asstalker_ai_fullcontrollable (- (Variables|/Game/GameBPs/Blueprints/StalkerAI_fullcontrollable.StalkerAI_fullcontrollable_C|GetHealth _asstalker_ai_fullcontrollable) 2e+01))
            (goto _label)))
        (else
          (Variables|/Game/GameBPs/Blueprints/ThirdPersonCharacterTT.ThirdPersonCharacterTT_C|SetTotalHealth _asthird_person_character_tt (- (Variables|/Game/GameBPs/Blueprints/ThirdPersonCharacterTT.ThirdPersonCharacterTT_C|GetTotalHealth _asthird_person_character_tt) 1))
          (Variables|Default|SetCanAttack false)
          (CallFunction|AttackDelay))))))

(event Custom|Attack%20Delay
  ;[1 1 1] Attack Delay
  (Utilities|FlowControl|Delay 2.0)
  (Variables|Default|SetCanAttack true))

(event Custom|Update%20Score
  (bind _outactors (Actor|GetAllActorsOfClass "/Game/GameBPs/Blueprints/ThirdPersonCharacterTT.ThirdPersonCharacterTT_C"))
  (bind _asthird_person_character_tt (Utilities|Casting|CastToThirdPersonCharacterTT (Utilities|Array|Get(acopy) _outactors)))
  (Variables|/Game/GameBPs/Blueprints/ThirdPersonCharacterTT.ThirdPersonCharacterTT_C|SetScore _asthird_person_character_tt (+ 100 (Variables|/Game/GameBPs/Blueprints/ThirdPersonCharacterTT.ThirdPersonCharacterTT_C|GetScore _asthird_person_character_tt))))

(event Custom|HeadHitCryo
  (bind _mesh (Variables|Character|GetMesh))
  (bind _mesh_2 (Variables|Character|GetMesh))
  (Variables|Default|SetHealth (- (Variables|Default|GetHealth) 75.0))
  (bind _outactors (Actor|GetAllActorsOfClass "/Game/GameBPs/Blueprints/ThirdPersonCharacterTT.ThirdPersonCharacterTT_C"))
  (bind _asthird_person_character_tt (Utilities|Casting|CastToThirdPersonCharacterTT (Utilities|Array|Get(acopy) _outactors)))
  (Variables|/Game/GameBPs/Blueprints/ThirdPersonCharacterTT.ThirdPersonCharacterTT_C|SetScore _asthird_person_character_tt (+ (Variables|/Game/GameBPs/Blueprints/ThirdPersonCharacterTT.ThirdPersonCharacterTT_C|GetScore _asthird_person_character_tt) 1))
  (Variables|/Script/Engine.CharacterMovementComponent|SetMaxWalkSpeed (Variables|Character|GetCharacterMovement) 1.5e+02)
  (Rendering|Material|SetMaterial _mesh_2 1 "/Game/Textures/Cyan.Cyan")
  (Rendering|Material|SetMaterial _mesh_2 0 "/Game/Textures/Cyan.Cyan")
  (Utilities|FlowControl|Delay 3.0)
  (Variables|/Script/Engine.CharacterMovementComponent|SetMaxWalkSpeed (Variables|Character|GetCharacterMovement) 5e+02)
  (Rendering|Material|SetMaterial _mesh 0 "/Game/Characters/Character/Materials/M_UE4Man_Body.M_UE4Man_Body")
  (Rendering|Material|SetMaterial _mesh 1 "/Game/Characters/Character/Materials/M_UE4Man_ChestLogo.M_UE4Man_ChestLogo"))

(event Custom|RangeFinder
  ;[1 1 1] Attack Range
  (if (<= (Math|Vector|VectorLength (- (Transformation|GetActorLocation (Game|Player|GetPlayerPawn 0)) (Transformation|GetActorLocation))) 3e+02)
    (Variables|Default|SetInAttackRange true)
    (if (Variables|Default|GetInAttackRange)
      (Development|PrintString "InRange")
      (CallFunction|AttackPlayer))))

(event Custom|MassFreeze
  (bind _mesh (Variables|Character|GetMesh))
  (bind _mesh_2 (Variables|Character|GetMesh))
  ;[0 0.8898 1] MassFreeze
  (Variables|/Script/Engine.CharacterMovementComponent|SetMaxWalkSpeed (Variables|Character|GetCharacterMovement) 1.5e+02)
  (Rendering|Material|SetMaterial _mesh 1 "/Game/Textures/Cyan.Cyan")
  (Rendering|Material|SetMaterial _mesh 0 "/Game/Textures/Cyan.Cyan")
  (Utilities|FlowControl|Delay 15.0)
  (Variables|/Script/Engine.CharacterMovementComponent|SetMaxWalkSpeed (Variables|Character|GetCharacterMovement) 5e+02)
  (Rendering|Material|SetMaterial _mesh_2 0 "/Game/Characters/Character/Materials/M_UE4Man_Body.M_UE4Man_Body")
  (Rendering|Material|SetMaterial _mesh_2 1 "/Game/Characters/Character/Materials/M_UE4Man_ChestLogo.M_UE4Man_ChestLogo"))

(event Custom|Advance%20towards%20player
  (CallFunction|RangeFinder)
  (CallFunction|HealthCheck)
  (AI|AIMoveTo self "0, 0, 0" (Game|GetPlayerCharacter 0) 5e+01 false))

(event Custom|Health%20Check
  (bind _returnvalue (Transformation|GetActorLocation))
  (bind _returnvalue_2 (Math|Conversions|ToTransform(Vector) _returnvalue))
  (if (<= (Variables|Default|GetHealth) 0.0)
    (CallFunction|UpdateScore)
    (Actor|DestroyActor)
    (switch int (Math|Random|RandomIntegerinRange 0 12)
      (:0
        (Game|SpawnActorfromClass "/Game/Blueprints/AmmoBoxSmall.AmmoBoxSmall_C" _returnvalue_2 "Undefined" 0 0))
      (:1
        (Game|SpawnActorfromClass "/Game/Blueprints/HealthBoxSmall.HealthBoxSmall_C" _returnvalue_2 "Undefined" 0 0))
      (:2
        (Game|SpawnActorfromClass "/Game/Blueprints/EnergyBoxSmall.EnergyBoxSmall_C" _returnvalue_2 "Undefined" 0 0)))))

(event Game|Damage|EventRadialDamage
  (params (DamageReceived :type Float%20%28single-precision%29) (DamageType :type Damage%20Type%20Object%20Reference) (Origin :type Vector :default "0, 0, 0") (HitInfo :type Hit%20Result%20Structure%20%28by%20ref%29) (InstigatedBy :type Controller%20Object%20Reference) (DamageCauser :type Actor%20Object%20Reference))
  (Variables|Default|SetDamageType DamageType)
  (Variables|Default|SetHealth (- (Variables|Default|GetHealth) DamageReceived)))

(event EventBeginPlay
  (CallFunction|AdvanceTowardsPlayer))

(event EventTick
  (params (DeltaSeconds :type Float%20%28single-precision%29))
  (CallFunction|AdvanceTowardsPlayer))

(event Game|Damage|EventAnyDamage
  (params (Damage :type Float%20%28single-precision%29) (DamageType :type Damage%20Type%20Object%20Reference) (InstigatedBy :type Controller%20Object%20Reference) (DamageCauser :type Actor%20Object%20Reference))
  (Variables|Default|SetHealth (- (Variables|Default|GetHealth) Damage)))

(event Collision|EventHit
  (params (MyComp :type Primitive%20Component%20Object%20Reference) (Other :type Actor%20Object%20Reference) (OtherComp :type Primitive%20Component%20Object%20Reference) (bSelfMoved :type Boolean) (HitLocation :type Vector :default "0, 0, 0") (HitNormal :type Vector :default "0, 0, 0") (NormalImpulse :type Vector :default "0, 0, 0") (Hit :type Hit%20Result%20Structure%20%28by%20ref%29))
  (bind _mesh (Variables|Character|GetMesh))
  (bind _charactermovement (Variables|Character|GetCharacterMovement))
  (bind _mesh_2 (Variables|Character|GetMesh))
  (Utilities|Casting|CastToCryoProjectileNEW Other)
  (Variables|/Script/Engine.CharacterMovementComponent|SetMaxWalkSpeed _charactermovement 1.5e+02)
  (Rendering|Material|SetMaterial _mesh_2 0 "/Game/Textures/Cyan.Cyan")
  (Rendering|Material|SetMaterial _mesh_2 1 "/Game/Textures/Cyan.Cyan")
  (Utilities|FlowControl|Delay 1e+01)
  (Variables|/Script/Engine.CharacterMovementComponent|SetMaxWalkSpeed _charactermovement 5e+02)
  (Rendering|Material|SetMaterial _mesh 0 "/Game/Characters/Character/Materials/M_UE4Man_Body.M_UE4Man_Body")
  (Rendering|Material|SetMaterial _mesh 1 "/Game/Characters/Character/Materials/M_UE4Man_ChestLogo.M_UE4Man_ChestLogo"))

(fn ConstructionScript)