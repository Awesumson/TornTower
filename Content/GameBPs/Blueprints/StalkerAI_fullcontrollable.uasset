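; Player-pilotable Stalker combat vehicle that hands possession back to ThirdPersonCharacterTT on exit or when destroyed.
; Input drives movement, sprint with flame effects, a Gate-throttled cannon, looping twin-barrel sidegun and up to three timed ally mines.
; Tick updates the armour text and checks health, exploding at zero; damage and cryo events reduce health or temporarily slow it.
; Auto-turret targeting and firing logic is left stubbed or disconnected.
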(event Custom|TurretRotation
  ;[1 1 1] Rotation & Track Player
)

(event Custom|Text%20Face%20Player
  (Transformation|SetWorldRotation (Variables|Default|GetTextRender) (Math|Conversions|RotationFromXVector (Math|Vector|RotateVector (Math|Vector|Normalize (* (- (Transformation|GetWorldLocation (Variables|Default|GetCamera)) (Transformation|GetActorLocation)) "1.000000,1.000000,0.000000")) "0, 0, 0")) false false))

(event Custom|Exit%20Vehicle
  ;[1 0.008451 0] Exit Stalker
  (bind _outactors (Actor|GetAllActorsOfClass "/Game/GameBPs/Blueprints/ThirdPersonCharacterTT.ThirdPersonCharacterTT_C"))
  (bind _asthird_person_character_tt (Utilities|Casting|CastToThirdPersonCharacterTT (Utilities|Array|Get(acopy) _outactors)))
  (Transformation|SetActorLocation _asthird_person_character_tt (+ (Variables|Default|GetStoreLocation) "300.000000,50.000000, 0") false false)
  (Utilities|FlowControl|Delay 0.1)
  (Pawn|Possess (Game|GetPlayerController 0) _asthird_person_character_tt)
  (Rendering|SetActorHiddenInGame _asthird_person_character_tt false)
  (Variables|/Game/GameBPs/Blueprints/ThirdPersonCharacterTT.ThirdPersonCharacterTT_C|SetInVehicle_2 _asthird_person_character_tt false)
  (Variables|Default|SetPossessed false)
  (Variables|Default|SetCanFire false)
  (CallFunction|RemoveAllyTag)
  (bind _foundwidgets (Widget|GetAllWidgetsOfClass "/Game/Interfaces/StalkerControls.StalkerControls_C" true))
  (bind _asstalker_controls (Utilities|Casting|CastToStalkerControls (Utilities|Array|Get(acopy) _foundwidgets)))
  (Widget|RemovefromParent _asstalker_controls))

(event Custom|ShotCooldown
  (bind _barrels (Variables|Default|GetBarrels))
  (bind _returnvalue (Transformation|GetSocketTransform _barrels "Barrel" "RTS_World"))
  (Utilities|FlowControl|Gate false) ; enters at Close
)

(event Custom|HeadHit
  (Variables|Default|SetHealth (- (Variables|Default|GetHealth) 1e+02))
  (bind _outactors (Actor|GetAllActorsOfClass "/Game/GameBPs/Blueprints/ThirdPersonCharacterTT.ThirdPersonCharacterTT_C"))
  (bind _asthird_person_character_tt (Utilities|Casting|CastToThirdPersonCharacterTT (Utilities|Array|Get(acopy) _outactors)))
  (Variables|/Game/GameBPs/Blueprints/ThirdPersonCharacterTT.ThirdPersonCharacterTT_C|SetScore _asthird_person_character_tt (+ (Variables|/Game/GameBPs/Blueprints/ThirdPersonCharacterTT.ThirdPersonCharacterTT_C|GetScore _asthird_person_character_tt) 1)))

(event Custom|AttackPlayer
  ;[1 1 1] Attack
  (if (Variables|Default|GetInAttackRange)
    (if (Variables|Default|GetCanAttack)
      (bind _outactors (Actor|GetAllActorsOfClass "/Game/GameBPs/Blueprints/ThirdPersonCharacterTT.ThirdPersonCharacterTT_C"))
      (bind _asthird_person_character_tt (Utilities|Casting|CastToThirdPersonCharacterTT (Utilities|Array|Get(acopy) _outactors)))
      (Variables|/Game/GameBPs/Blueprints/ThirdPersonCharacterTT.ThirdPersonCharacterTT_C|SetTotalHealth _asthird_person_character_tt (- (Variables|/Game/GameBPs/Blueprints/ThirdPersonCharacterTT.ThirdPersonCharacterTT_C|GetTotalHealth _asthird_person_character_tt) 1))
      (Variables|Default|SetCanAttack false)
      (CallFunction|AttackDelay))))

(event Custom|FireSecondary
  (if (Variables|Default|GetIs%20Firing%20Sub)
    (Audio|Components|Audio|Play (Variables|Default|GetAudio_sidegun) 0.0)
    (Game|SpawnActorfromClass "/Game/Projectile_stalker_sidegun.Projectile_stalker_sidegun_C" (Transformation|GetSocketTransform (Variables|Default|GetSideGun) "Barrel_1" "RTS_World") "Undefined" 0 0)
    (Game|SpawnActorfromClass "/Game/Projectile_stalker_sidegun.Projectile_stalker_sidegun_C" (Transformation|GetSocketTransform (Variables|Default|GetSideGun) "Barrel_2" "RTS_World") "Undefined" 0 0)
    (Utilities|FlowControl|Delay (Variables|Default|GetFireRateSecondary))
    (CallFunction|FireSecondary)))

(event Custom|Find%20Player%20Range
  (bind _staticmesh (Variables|Default|GetStaticMesh))
  (bind _returnvalue (Transformation|GetWorldRotation _staticmesh))
  (bind (_roll _pitch _yaw) (Math|Rotator|BreakRotator _returnvalue))
  ;[1 1 1] Find Player Range
  (bind _nearest (CallFunction|FindClosestTarget))
  (bind _output_get (Variables|Default|SetNearestTargetDistance (Transformation|GetDistanceTo self _nearest)))
  (if (< _output_get (Variables|Default|GetAttackRange))
    (Variables|Default|SetInRange true)
    (else
      (Variables|Default|SetInRange false)
      (Transformation|SetWorldRotation (Variables|Default|GetBarrels) (Math|Rotator|MakeRotator _roll _pitch (- _yaw 9e+01)) false false))))

(event Custom|ShootAtPlayer
  (if (Variables|Default|GetInRange)
    (if (Variables|Default|GetCanFire)
      _)))

(event Custom|ArmourRegen
  ;[0.3955 0.9801 1] Armour Regen
  (if (Variables|Default|GetPossessed)
    (Utilities|FlowControl|Delay 0.25)
    (if (< (Variables|Default|GetHealth) 1e+03)
      (Variables|Default|SetHealth (+ (Variables|Default|GetHealth) 1.0))
      (CallFunction|ArmourRegen))))

(event Custom|Attack%20Delay
  ;[1 1 1] Attack Delay
  (Utilities|FlowControl|Delay 2.0)
  (Variables|Default|SetCanAttack true))

(event Custom|CanFireCheck
  (if (<= (Variables|Default|GetNearestTargetDistance) 0.0)
    (Variables|Default|SetCanFire false)
    (Variables|Default|SetCanRotateTurret false)
    (else
      (Variables|Default|SetCanFire true)
      (Variables|Default|SetCanRotateTurret true))))

(event Custom|Update%20Score
  (bind _outactors (Actor|GetAllActorsOfClass "/Game/GameBPs/Blueprints/ThirdPersonCharacterTT.ThirdPersonCharacterTT_C"))
  (bind _asthird_person_character_tt (Utilities|Casting|CastToThirdPersonCharacterTT (Utilities|Array|Get(acopy) _outactors)))
  (Variables|/Game/GameBPs/Blueprints/ThirdPersonCharacterTT.ThirdPersonCharacterTT_C|SetScore _asthird_person_character_tt (+ 500 (Variables|/Game/GameBPs/Blueprints/ThirdPersonCharacterTT.ThirdPersonCharacterTT_C|GetScore _asthird_person_character_tt))))

(event Custom|DeductMineCount
  (params (DestroyedActor :type Actor%20Object%20Reference))
  (Variables|Default|SetMinesSpawned (- (Variables|Default|GetMinesSpawned) 1)))

(event Custom|TargetDebug
  ;[1 1 1] target laser
  (if (Variables|Default|GetCanFire)
    (Rendering|Debug|DrawDebugLine (Transformation|GetWorldLocation (Variables|Default|GetBarrels)) (Transformation|GetWorldLocation (Variables|/Script/Engine.Actor|GetRootComponent (Variables|Default|GetNearestTarget))) "(R=1.000000,G=0.026519,B=0.000000,A=1.000000)" 0.1 1.0)))

(event Custom|HeadHitCryo
  (bind _mesh (Variables|Character|GetMesh))
  (bind _mesh_2 (Variables|Character|GetMesh))
  (Variables|Default|SetHealth (- (Variables|Default|GetHealth) 75.0))
  (bind _outactors (Actor|GetAllActorsOfClass "/Game/GameBPs/Blueprints/ThirdPersonCharacterTT.ThirdPersonCharacterTT_C"))
  (bind _asthird_person_character_tt (Utilities|Casting|CastToThirdPersonCharacterTT (Utilities|Array|Get(acopy) _outactors)))
  (Variables|/Game/GameBPs/Blueprints/ThirdPersonCharacterTT.ThirdPersonCharacterTT_C|SetScore _asthird_person_character_tt (+ (Variables|/Game/GameBPs/Blueprints/ThirdPersonCharacterTT.ThirdPersonCharacterTT_C|GetScore _asthird_person_character_tt) 1))
  (Variables|/Script/Engine.CharacterMovementComponent|SetMaxWalkSpeed (Variables|Character|GetCharacterMovement) 1.5e+02)
  (Rendering|Material|SetMaterial _mesh_2 1 "/Game/Textures/Cyan.Cyan")
  (Rendering|Material|SetMaterial _mesh_2 0 "/Game/Textures/Cyan.Cyan")
  (Utilities|FlowControl|Delay 3.0)
  (Variables|/Script/Engine.CharacterMovementComponent|SetMaxWalkSpeed (Variables|Character|GetCharacterMovement) 5e+02)
  (Rendering|Material|SetMaterial _mesh 0 "/Game/Characters/Character/Materials/M_UE4Man_Body.M_UE4Man_Body")
  (Rendering|Material|SetMaterial _mesh 1 "/Game/Characters/Character/Materials/M_UE4Man_ChestLogo.M_UE4Man_ChestLogo"))

(event Custom|RangeFinder
  ;[1 1 1] Attack Range
  (if (<= (Math|Vector|VectorLength (- (Transformation|GetActorLocation (Game|Player|GetPlayerPawn 0)) (Transformation|GetActorLocation))) 3e+02)
    (Variables|Default|SetInAttackRange true)
    (if (Variables|Default|GetInAttackRange)
      (Development|PrintString "InRange")
      (CallFunction|AttackPlayer))))

(event Custom|MassFreeze
  (bind _mesh (Variables|Character|GetMesh))
  (bind _mesh_2 (Variables|Character|GetMesh))
  ;[0 0.8898 1] MassFreeze
  (Variables|/Script/Engine.CharacterMovementComponent|SetMaxWalkSpeed (Variables|Character|GetCharacterMovement) 1.5e+02)
  (Rendering|Material|SetMaterial _mesh 1 "/Game/Textures/Cyan.Cyan")
  (Rendering|Material|SetMaterial _mesh 0 "/Game/Textures/Cyan.Cyan")
  (Utilities|FlowControl|Delay 15.0)
  (Variables|/Script/Engine.CharacterMovementComponent|SetMaxWalkSpeed (Variables|Character|GetCharacterMovement) 5e+02)
  (Rendering|Material|SetMaterial _mesh_2 0 "/Game/Characters/Character/Materials/M_UE4Man_Body.M_UE4Man_Body")
  (Rendering|Material|SetMaterial _mesh_2 1 "/Game/Characters/Character/Materials/M_UE4Man_ChestLogo.M_UE4Man_ChestLogo"))

(event Custom|EjectPlayer
  ;[1 0.008451 0] Exit Stalker
  (bind _outactors (Actor|GetAllActorsOfClass "/Game/GameBPs/Blueprints/ThirdPersonCharacterTT.ThirdPersonCharacterTT_C"))
  (bind _asthird_person_character_tt (Utilities|Casting|CastToThirdPersonCharacterTT (Utilities|Array|Get(acopy) _outactors)))
  (Transformation|SetActorLocation _asthird_person_character_tt (+ (Variables|Default|GetStoreLocation) "300.000000,50.000000, 0") false false)
  (Utilities|FlowControl|Delay 0.1)
  (Pawn|Possess (Game|GetPlayerController 0) _asthird_person_character_tt)
  (Rendering|SetActorHiddenInGame _asthird_person_character_tt false)
  (Variables|/Game/GameBPs/Blueprints/ThirdPersonCharacterTT.ThirdPersonCharacterTT_C|SetInVehicle_2 _asthird_person_character_tt false)
  (Variables|Default|SetPossessed false)
  (Variables|Default|SetCanFire false)
  (CallFunction|RemoveAllyTag)
  (bind _foundwidgets (Widget|GetAllWidgetsOfClass "/Game/Interfaces/StalkerControls.StalkerControls_C" true))
  (bind _asstalker_controls (Utilities|Casting|CastToStalkerControls (Utilities|Array|Get(acopy) _foundwidgets)))
  (Widget|RemovefromParent _asstalker_controls))

(event Custom|CanShootAgain
  (bind _barrels (Variables|Default|GetBarrels))
  (bind _returnvalue (Transformation|GetSocketTransform _barrels "Barrel" "RTS_World"))
  (Utilities|FlowControl|Gate false) ; enters at Open
)

(event Custom|Health%20Check
  (if (<= (Variables|Default|GetHealth) 0.0)
    (if (Variables|Default|GetPossessed)
      (CallFunction|EjectPlayer))
    (Utilities|FlowControl|Delay 0.5)
    (Actor|DestroyActor)
    (Effects|SpawnEmitteratLocation "/Game/StarterContent/Particles/P_Explosion.P_Explosion" (Transformation|GetActorLocation) "0, 0, 0" "7.000000,7.000000,7.000000")))

(event Game|Damage|EventRadialDamage
  (params (DamageReceived :type Float%20%28single-precision%29) (DamageType :type Damage%20Type%20Object%20Reference) (Origin :type Vector :default "0, 0, 0") (HitInfo :type Hit%20Result%20Structure%20%28by%20ref%29) (InstigatedBy :type Controller%20Object%20Reference) (DamageCauser :type Actor%20Object%20Reference))
  (Variables|Default|SetDamageType DamageType)
  (Variables|Default|SetHealth (- (Variables|Default|GetHealth) DamageReceived)))

(event EventBeginPlay
  (CallFunction|ShootatPlayer)
  (CallFunction|CanShootAgain))

(event EventTick
  (params (DeltaSeconds :type Float%20%28single-precision%29))
  (Variables|Default|SetStoreLocation (Transformation|GetActorLocation))
  (CallFunction|HealthCheck)
  (CallFunction|TextFacePlayer)
  (Rendering|Components|TextRender|SetText (Variables|Default|GetTextRender) (Utilities|Text|ToText(String) (Utilities|String|Append "Armour: " (Utilities|String|ToString(Float) (Variables|Default|GetHealth))))))

(event Game|Damage|EventAnyDamage
  (params (Damage :type Float%20%28single-precision%29) (DamageType :type Damage%20Type%20Object%20Reference) (InstigatedBy :type Controller%20Object%20Reference) (DamageCauser :type Actor%20Object%20Reference))
  (Variables|Default|SetHealth (- (Variables|Default|GetHealth) Damage)))

(event Collision|EventHit
  (params (MyComp :type Primitive%20Component%20Object%20Reference) (Other :type Actor%20Object%20Reference) (OtherComp :type Primitive%20Component%20Object%20Reference) (bSelfMoved :type Boolean) (HitLocation :type Vector :default "0, 0, 0") (HitNormal :type Vector :default "0, 0, 0") (NormalImpulse :type Vector :default "0, 0, 0") (Hit :type Hit%20Result%20Structure%20%28by%20ref%29))
  (bind _mesh (Variables|Character|GetMesh))
  (bind _charactermovement (Variables|Character|GetCharacterMovement))
  (bind _mesh_2 (Variables|Character|GetMesh))
  (Utilities|Casting|CastToCryoProjectileNEW Other)
  (Variables|/Script/Engine.CharacterMovementComponent|SetMaxWalkSpeed _charactermovement 1.5e+02)
  (Rendering|Material|SetMaterial _mesh_2 0 "/Game/Textures/Cyan.Cyan")
  (Rendering|Material|SetMaterial _mesh_2 1 "/Game/Textures/Cyan.Cyan")
  (Utilities|FlowControl|Delay 1e+01)
  (Variables|/Script/Engine.CharacterMovementComponent|SetMaxWalkSpeed _charactermovement 5e+02)
  (Rendering|Material|SetMaterial _mesh 0 "/Game/Characters/Character/Materials/M_UE4Man_Body.M_UE4Man_Body")
  (Rendering|Material|SetMaterial _mesh 1 "/Game/Characters/Character/Materials/M_UE4Man_ChestLogo.M_UE4Man_ChestLogo"))

(event Input|ActionEvents|InputActionAltFire
  (params (Key :type Key%20Structure))
  (:Pressed
    (Variables|Default|SetIs%20Firing%20Sub true)
    (CallFunction|FireSecondary))
  (:Released
    (Variables|Default|SetIs%20Firing%20Sub false)))

(event Input|ActionEvents|InputActionFire
  (params (Key :type Key%20Structure))
  (bind _barrels (Variables|Default|GetBarrels))
  (bind _returnvalue (Transformation|GetSocketTransform _barrels "Barrel" "RTS_World"))
  (:Pressed
    (Utilities|FlowControl|Gate false
      (:Exit
        (Audio|Components|Audio|Play (Variables|Default|GetAudio_cannon) 0.0)
        (Game|SpawnActorfromClass "/Game/Projectile_ally_explosion.Projectile_ally_explosion_C" _returnvalue "Undefined" 0 0)
        (Effects|SpawnEmitteratLocation "/Game/StarterContent/Particles/P_Cannon_muzzleflash.P_Cannon_muzzleflash" (.Location (Math|Transform|BreakTransform _returnvalue)))
        (CallFunction|ShotCooldown)
        (Utilities|FlowControl|RetriggerableDelay (Variables|Default|GetFireRateCANNON))
        (CallFunction|CanShootAgain)))))

(event Input|ActionEvents|InputActionInteract
  (params (Key :type Key%20Structure))
  (:Pressed
    (CallFunction|ExitVehicle)))

(event Input|ActionEvents|InputActionSpawnMine(AsStalker)
  (params (Key :type Key%20Structure))
  (:Pressed
    (if (< (Variables|Default|GetMinesSpawned) 3)
      (bind _returnvalue (Game|SpawnActorfromClass "/Game/Blueprints/StalkerMine_ally.StalkerMine_ally_C" (Math|Conversions|ToTransform(Vector) (Transformation|GetWorldLocation (Variables|Default|GetMineSpawnloc))) "Undefined" 0 0))
      (Variables|Default|SetMinesSpawned (+ (Variables|Default|GetMinesSpawned) 1))
      (Game|BindEventtoOnDestroyed _returnvalue (delegate Custom|DeductMineCount))
      (Actor|SetLifeSpan (stale Custom|DeductMineCount DestroyedActor) 9e+01))))

(event Input|ActionEvents|InputActionSprint
  (params (Key :type Key%20Structure))
  (bind _charactermovement (Variables|Character|GetCharacterMovement))
  (:Pressed
    (Variables|/Script/Engine.CharacterMovementComponent|SetMaxWalkSpeed _charactermovement 3e+03)
    (Development|SetHiddeninGame (Variables|Default|GetFire1) false false)
    (Development|SetHiddeninGame (Variables|Default|GetFire2) false false))
  (:Released
    (Variables|/Script/Engine.CharacterMovementComponent|SetMaxWalkSpeed _charactermovement 1.3e+03)
    (Development|SetHiddeninGame (Variables|Default|GetFire1) true false)
    (Development|SetHiddeninGame (Variables|Default|GetFire2) true false)))

(event Input|AxisEvents|InputAxisLookUp
  (params (AxisValue :type Float%20%28single-precision%29))
  (Pawn|Input|AddControllerPitchInput AxisValue))

(event Input|AxisEvents|InputAxisTurn
  (params (AxisValue :type Float%20%28single-precision%29))
  (Pawn|Input|AddControllerYawInput AxisValue))

(event Input|AxisEvents|InputAxisMoveForward
  (params (AxisValue :type Float%20%28single-precision%29))
  (Pawn|Input|AddMovementInput (Math|Vector|GetForwardVector (Math|Rotator|MakeRotator 0.0 0.0 (.Yaw (Math|Rotator|BreakRotator (Pawn|GetControlRotation :!class /Script/Engine.Pawn))))) AxisValue false))

(event Input|AxisEvents|InputAxisMoveRight
  (params (AxisValue :type Float%20%28single-precision%29))
  (Pawn|Input|AddMovementInput (Math|Vector|GetRightVector (Math|Rotator|MakeRotator 0.0 0.0 (.Yaw (Math|Rotator|BreakRotator (Pawn|GetControlRotation :!class /Script/Engine.Pawn))))) AxisValue false))

(fn ConstructionScript)

(fn FindClosestTarget
  (bind _outactors (Actor|GetAllActorswithTag "Enemy"))
  (for _array_element _outactors
    (if (< (Transformation|GetDistanceTo _array_element) (Variables|Default|GetAttackRange))
      (bind _output_get (Variables|Default|SetNearestTarget _array_element))))
  (return _output_get))

(fn AddAllyTag
  (Utilities|Array|Add (Variables|Actor|GetTags) (Variables|Default|GetAllyTag))
  (return))

(fn RemoveAllyTag
  (Utilities|Array|RemoveItem (Variables|Actor|GetTags) (Variables|Default|GetAllyTag))
  (return))