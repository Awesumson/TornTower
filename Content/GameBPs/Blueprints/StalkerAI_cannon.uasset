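; Stalker cannon enemy AI that roams to random points around the player, shelling Ally-tagged actors and dropping up to three mines.
; Tick rotates the barrels toward an in-range ally, while self-retriggering delay loops drive firing, movement and mine spawning.
; Movement updates also trigger close-range player damage.
; Hit events handle damage and cryo slows with material swaps; death awards score and drops a repair kit or care package.
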(event Custom|TurretRotation
  (bind _barrels (Variables|Default|GetBarrels))
  (bind _nearesttarget (Variables|Default|GetNearestTarget))
  (bind _returnvalue (Transformation|GetWorldLocation _barrels))
  (bind _returnvalue_2 (Transformation|GetActorLocation _nearesttarget))
  (bind _returnvalue_3 (Math|Rotator|FindLookatRotation _returnvalue _returnvalue_2))
  (bind (_roll _pitch _yaw) (Math|Rotator|BreakRotator _returnvalue_3))
  ;[1 1 1] Rotation & Track Player
  (if (Variables|Default|GetInRange)
    (Transformation|SetWorldRotation (Variables|Default|GetBarrels) (Math|Interpolation|RInterpTo (Transformation|GetWorldRotation (Variables|Default|GetBarrels)) (Math|Rotator|MakeRotator 0.0 _pitch _yaw) (Variables|Default|GetDeltaTime) (Variables|Default|GetRotationSpeed)) false false)))

(event Custom|Find%20Player%20Range
  ;[1 1 1] Find Player Range
  (bind _nearest (CallFunction|FindClosestTarget))
  (Variables|Default|SetNearestTargetDistance (Transformation|GetDistanceTo self _nearest))
  (if (< (Transformation|GetDistanceTo self _nearest) (Variables|Default|GetAttackRange))
    (Variables|Default|SetInRange true)
    (else
      (Variables|Default|SetInRange false))))

(event Custom|HeadHit
  (Variables|Default|SetHealth (- (Variables|Default|GetHealth) 1e+02))
  (bind _outactors (Actor|GetAllActorsOfClass "/Game/GameBPs/Blueprints/ThirdPersonCharacterTT.ThirdPersonCharacterTT_C"))
  (bind _asthird_person_character_tt (Utilities|Casting|CastToThirdPersonCharacterTT (Utilities|Array|Get(acopy) _outactors)))
  (Variables|/Game/GameBPs/Blueprints/ThirdPersonCharacterTT.ThirdPersonCharacterTT_C|SetScore _asthird_person_character_tt (+ (Variables|/Game/GameBPs/Blueprints/ThirdPersonCharacterTT.ThirdPersonCharacterTT_C|GetScore _asthird_person_character_tt) 1)))

(event Custom|AttackPlayer
  ;[1 1 1] Attack
  (if (Variables|Default|GetInAttackRange)
    (if (Variables|Default|GetCanAttack)
      (bind _outactors (Actor|GetAllActorsOfClass "/Game/GameBPs/Blueprints/ThirdPersonCharacterTT.ThirdPersonCharacterTT_C"))
      (bind _asthird_person_character_tt (Utilities|Casting|CastToThirdPersonCharacterTT (Utilities|Array|Get(acopy) _outactors)))
      (Variables|/Game/GameBPs/Blueprints/ThirdPersonCharacterTT.ThirdPersonCharacterTT_C|SetTotalHealth _asthird_person_character_tt (- (Variables|/Game/GameBPs/Blueprints/ThirdPersonCharacterTT.ThirdPersonCharacterTT_C|GetTotalHealth _asthird_person_character_tt) 1))
      (Variables|Default|SetCanAttack false)
      (CallFunction|AttackDelay))))

(event Custom|ShootAtPlayer
  (bind _barrels (Variables|Default|GetBarrels))
  (bind _returnvalue (Transformation|GetSocketTransform _barrels "Barrel" "RTS_World"))
  (if (Variables|Default|GetInRange)
    (if (Variables|Default|GetCanFire)
      (Audio|Components|Audio|Play (Variables|Default|GetAudio) 0.0)
      (Game|SpawnActorfromClass "/Game/Projectile_Enemy_explosion.Projectile_Enemy_explosion_C" _returnvalue "Undefined" 0 0)
      (Effects|SpawnEmitteratLocation "/Game/StarterContent/Particles/P_Cannon_muzzleflash.P_Cannon_muzzleflash" (.Location (Math|Transform|BreakTransform _returnvalue)))
      (Utilities|FlowControl|RetriggerableDelay (Variables|Default|GetFireRate))
      (CallFunction|ShootatPlayer)
      (else
        (Utilities|FlowControl|RetriggerableDelay 0.5 :!label _label)
        (CallFunction|ShootatPlayer)))
    (else
      (goto _label))))

(event Custom|Attack%20Delay
  ;[1 1 1] Attack Delay
  (Utilities|FlowControl|Delay 2.0)
  (Variables|Default|SetCanAttack true))

(event Custom|CanFireCheck
  (if (<= (Variables|Default|GetNearestTargetDistance) 0.0)
    (Variables|Default|SetCanFire false)
    (else
      (Variables|Default|SetCanFire true))))

(event Custom|Update%20Score
  (bind _outactors (Actor|GetAllActorsOfClass "/Game/GameBPs/Blueprints/ThirdPersonCharacterTT.ThirdPersonCharacterTT_C"))
  (bind _asthird_person_character_tt (Utilities|Casting|CastToThirdPersonCharacterTT (Utilities|Array|Get(acopy) _outactors)))
  (Variables|/Game/GameBPs/Blueprints/ThirdPersonCharacterTT.ThirdPersonCharacterTT_C|SetScore _asthird_person_character_tt (+ 500 (Variables|/Game/GameBPs/Blueprints/ThirdPersonCharacterTT.ThirdPersonCharacterTT_C|GetScore _asthird_person_character_tt))))

(event Custom|DeductMineCount
  (params (DestroyedActor :type Actor%20Object%20Reference))
  (Variables|Default|SetMinesSpawned (- (Variables|Default|GetMinesSpawned) 1)))

(event Custom|HeadHitCryo
  (bind _mesh (Variables|Character|GetMesh))
  (bind _mesh_2 (Variables|Character|GetMesh))
  (Variables|Default|SetHealth (- (Variables|Default|GetHealth) 75.0))
  (bind _outactors (Actor|GetAllActorsOfClass "/Game/GameBPs/Blueprints/ThirdPersonCharacterTT.ThirdPersonCharacterTT_C"))
  (bind _asthird_person_character_tt (Utilities|Casting|CastToThirdPersonCharacterTT (Utilities|Array|Get(acopy) _outactors)))
  (Variables|/Game/GameBPs/Blueprints/ThirdPersonCharacterTT.ThirdPersonCharacterTT_C|SetScore _asthird_person_character_tt (+ (Variables|/Game/GameBPs/Blueprints/ThirdPersonCharacterTT.ThirdPersonCharacterTT_C|GetScore _asthird_person_character_tt) 1))
  (Variables|/Script/Engine.CharacterMovementComponent|SetMaxWalkSpeed (Variables|Character|GetCharacterMovement) 1.5e+02)
  (Rendering|Material|SetMaterial _mesh_2 1 "/Game/Textures/Cyan.Cyan")
  (Rendering|Material|SetMaterial _mesh_2 0 "/Game/Textures/Cyan.Cyan")
  (Utilities|FlowControl|Delay 3.0)
  (Variables|/Script/Engine.CharacterMovementComponent|SetMaxWalkSpeed (Variables|Character|GetCharacterMovement) 5e+02)
  (Rendering|Material|SetMaterial _mesh 0 "/Game/Characters/Character/Materials/M_UE4Man_Body.M_UE4Man_Body")
  (Rendering|Material|SetMaterial _mesh 1 "/Game/Characters/Character/Materials/M_UE4Man_ChestLogo.M_UE4Man_ChestLogo"))

(event Custom|RangeFinder
  ;[1 1 1] Attack Range
  (if (<= (Math|Vector|VectorLength (- (Transformation|GetActorLocation (Game|Player|GetPlayerPawn 0)) (Transformation|GetActorLocation))) 3e+02)
    (Variables|Default|SetInAttackRange true)
    (if (Variables|Default|GetInAttackRange)
      (Development|PrintString "InRange")
      (CallFunction|AttackPlayer))))

(event Custom|MassFreeze
  (bind _mesh (Variables|Character|GetMesh))
  (bind _mesh_2 (Variables|Character|GetMesh))
  ;[0 0.8898 1] MassFreeze
  (Variables|/Script/Engine.CharacterMovementComponent|SetMaxWalkSpeed (Variables|Character|GetCharacterMovement) 1.5e+02)
  (Rendering|Material|SetMaterial _mesh 1 "/Game/Textures/Cyan.Cyan")
  (Rendering|Material|SetMaterial _mesh 0 "/Game/Textures/Cyan.Cyan")
  (Utilities|FlowControl|Delay 15.0)
  (Variables|/Script/Engine.CharacterMovementComponent|SetMaxWalkSpeed (Variables|Character|GetCharacterMovement) 5e+02)
  (Rendering|Material|SetMaterial _mesh_2 0 "/Game/Characters/Character/Materials/M_UE4Man_Body.M_UE4Man_Body")
  (Rendering|Material|SetMaterial _mesh_2 1 "/Game/Characters/Character/Materials/M_UE4Man_ChestLogo.M_UE4Man_ChestLogo"))

(event Custom|Advance%20towards%20player
  (bind _returnvalue (Game|GetPlayerCharacter 0))
  (bind _returnvalue_2 (Math|Random|RandomFloatinRange 5.0 9.0))
  (bind _returnvalue_3 (Transformation|GetActorLocation _returnvalue))
  (bind (_x _y _z) (Math|Vector|BreakVector _returnvalue_3))
  (CallFunction|RangeFinder)
  (CallFunction|HealthCheck)
  (bind _output_get (Variables|Default|SetTargetLocation (Math|Vector|MakeVector (+ (Math|Random|RandomFloatinRange -1.5e+03 1.5e+03) _x) (+ (Math|Random|RandomFloatinRange -1.5e+03 1.5e+03) _y) _z)))
  (AI|AIMoveTo self _output_get 0 5e+01 false
    (:OnSuccess
      _)
    (:OnFail
      _))
  (Utilities|FlowControl|Delay _returnvalue_2)
  (CallFunction|AdvanceTowardsPlayer)
  (Variables|Default|SetDebugDelay _returnvalue_2)
  (Rendering|Debug|DrawDebugPoint (Variables|Default|GetTargetLocation) 25.0 "(R=1.000000,G=0.000000,B=0.824260,A=1.000000)" (Variables|Default|GetDebugDelay)))

(event Custom|Health%20Check
  (bind _returnvalue (Transformation|GetActorLocation))
  (bind _returnvalue_2 (Math|Conversions|ToTransform(Vector) _returnvalue))
  (if (<= (Variables|Default|GetHealth) 0.0)
    (CallFunction|UpdateScore)
    (Actor|DestroyActor)
    (Effects|SpawnEmitteratLocation "/Game/StarterContent/Particles/P_Explosion.P_Explosion" (Transformation|GetActorLocation) "0, 0, 0" "7.000000,7.000000,7.000000")
    (switch int (Math|Random|RandomIntegerinRange 0 1)
      (:0
        (Game|SpawnActorfromClass "/Game/Blueprints/TowerRepairKit.TowerRepairKit_C" _returnvalue_2 "Undefined" 0 0))
      (:1
        (Game|SpawnActorfromClass "/Game/Blueprints/CarePackage.CarePackage_C" _returnvalue_2 "Undefined" 0 0)))))

(event Custom|Spawn%20Mines
  (if (< (Variables|Default|GetMinesSpawned) 3)
    (Utilities|FlowControl|Delay (Math|Random|RandomFloatinRange 15.0 3e+01))
    (bind _returnvalue (Game|SpawnActorfromClass "/Game/Blueprints/StalkerMine.StalkerMine_C" (Math|Conversions|ToTransform(Vector) (Transformation|GetWorldLocation (Variables|Default|GetMineSpawnloc))) "Undefined" 0 0))
    (Variables|Default|SetMinesSpawned (+ (Variables|Default|GetMinesSpawned) 1))
    (CallFunction|SpawnMines)
    (Game|BindEventtoOnDestroyed _returnvalue (delegate Custom|DeductMineCount))
    (Actor|SetLifeSpan _returnvalue 9e+01)
    (else
      (Utilities|FlowControl|Delay 1e+01)
      (CallFunction|SpawnMines))))

(event Custom|TurretController
  (params (DeltaSeconds :type Float%20%28single-precision%29))
  (Variables|Default|SetDeltaTime DeltaSeconds)
  (CallFunction|TurretRotation)
  (CallFunction|FindPlayerRange))

(event Game|Damage|EventRadialDamage
  (params (DamageReceived :type Float%20%28single-precision%29) (DamageType :type Damage%20Type%20Object%20Reference) (Origin :type Vector :default "0, 0, 0") (HitInfo :type Hit%20Result%20Structure%20%28by%20ref%29) (InstigatedBy :type Controller%20Object%20Reference) (DamageCauser :type Actor%20Object%20Reference))
  (Variables|Default|SetDamageType DamageType)
  (Variables|Default|SetHealth (- (Variables|Default|GetHealth) DamageReceived)))

(event EventBeginPlay
  (CallFunction|ShootatPlayer)
  (CallFunction|AdvanceTowardsPlayer)
  (CallFunction|SpawnMines))

(event EventTick
  (params (DeltaSeconds :type Float%20%28single-precision%29))
  (CallFunction|TurretController DeltaSeconds)
  (CallFunction|HealthCheck)
  (CallFunction|CanFireCheck)
  (Development|PrintString (Utilities|String|Append "Stalker (C) Health: " (Utilities|String|ToString(Float) (Variables|Default|GetHealth))))
  (Utilities|FlowControl|DoOnce false
    (:Completed
      (CallFunction|AdvanceTowardsPlayer))))

(event Game|Damage|EventAnyDamage
  (params (Damage :type Float%20%28single-precision%29) (DamageType :type Damage%20Type%20Object%20Reference) (InstigatedBy :type Controller%20Object%20Reference) (DamageCauser :type Actor%20Object%20Reference))
  (Variables|Default|SetHealth (- (Variables|Default|GetHealth) Damage)))

(event Collision|EventHit
  (params (MyComp :type Primitive%20Component%20Object%20Reference) (Other :type Actor%20Object%20Reference) (OtherComp :type Primitive%20Component%20Object%20Reference) (bSelfMoved :type Boolean) (HitLocation :type Vector :default "0, 0, 0") (HitNormal :type Vector :default "0, 0, 0") (NormalImpulse :type Vector :default "0, 0, 0") (Hit :type Hit%20Result%20Structure%20%28by%20ref%29))
  (bind _mesh (Variables|Character|GetMesh))
  (bind _charactermovement (Variables|Character|GetCharacterMovement))
  (bind _mesh_2 (Variables|Character|GetMesh))
  (Utilities|Casting|CastToCryoProjectileNEW Other)
  (Variables|/Script/Engine.CharacterMovementComponent|SetMaxWalkSpeed _charactermovement 1.5e+02)
  (Rendering|Material|SetMaterial _mesh_2 0 "/Game/Textures/Cyan.Cyan")
  (Rendering|Material|SetMaterial _mesh_2 1 "/Game/Textures/Cyan.Cyan")
  (Utilities|FlowControl|Delay 1e+01)
  (Variables|/Script/Engine.CharacterMovementComponent|SetMaxWalkSpeed _charactermovement 5e+02)
  (Rendering|Material|SetMaterial _mesh 0 "/Game/Characters/Character/Materials/M_UE4Man_Body.M_UE4Man_Body")
  (Rendering|Material|SetMaterial _mesh 1 "/Game/Characters/Character/Materials/M_UE4Man_ChestLogo.M_UE4Man_ChestLogo"))

(fn ConstructionScript)

(fn FindClosestTarget
  (bind _outactors (Actor|GetAllActorswithTag "Ally"))
  (for _array_element _outactors
    (if (< (Transformation|GetDistanceTo _array_element) (Variables|Default|GetAttackRange))
      (bind _output_get (Variables|Default|SetNearestTarget _array_element))))
  (return _output_get))